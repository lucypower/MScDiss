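; BP_FSMPawn is a Learning Agents pawn that holds finite-state-machine state for a shop that involves items, prices and discounts.
; On BeginPlay it registers itself with the LearningAgentsManager component on actors tagged FSMManager, printing a warning if none is found.
; RespawnPlayerPawn randomises the stats of the BP_FSMPlayerPawn in the scene, then resets its own FSM state, decision flags and shop lists.
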(event EventBeginPlay
  (|CallParentFunction)
  (bind _outactors (Actor|GetAllActorswithTag "FSMManager"))
  (for _array_element _outactors
    (Utilities|IsValid (Actor|GetComponentbyClass _array_element "/Script/LearningAgents.LearningAgentsManager")
      (:Is%20Valid
        (Class|LearningAgentsManager|AddAgent (Actor|GetComponentbyClass _array_element "/Script/LearningAgents.LearningAgentsManager") self)
        (Variables|Default|SetFoundManager? true))))
  (if (not (Variables|Default|GetFoundManager?))
    (Development|PrintString "Could not find Learning Agents manager. Did we forget to add one to the scene?")))

(fn ConstructionScript)

(fn RespawnPlayerPawn
  (bind _returnvalue (Actor|GetActorOfClass "/Game/Blueprints/FSMBPs/BP_FSMPlayerPawn.BP_FSMPlayerPawn_C"))
  (Class|FSMPlayerPawnComponent|RandomiseStats (Variables|/Game/Blueprints/FSMBPs/BP_FSMPlayerPawn.BP_FSMPlayerPawn_C|GetFSMPlayerPawn _returnvalue))
  (Variables|Default|SetObservedPlayer? false)
  (Variables|Default|SetResetShop? false)
  (Variables|Default|SetDecideDiscount? false)
  (Variables|Default|SetDecideItems? false)
  (Variables|Default|SetFSMState "NewEnumerator1")
  (Utilities|Array|Clear (Variables|Default|GetShopItemNames))
  (Utilities|Array|Clear (Variables|Default|GetShopItemPrices)))