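; BP_CollabAStarPawn is a Learning Agents pawn for the A* grid map, registering with the manager tagged AStarManager on BeginPlay.
; It caches wall spaces from BP_AStarMapGen and tracks wall touches through capsule overlaps.
; Raycast returns positions from eight horizontal traces at 45-degree steps.
; Reset teleports it to a fixed start and clears the touch count; its pawn-proximity check never rejects the spot.
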(event OnComponentBeginOverlap(CapsuleComponent)
  (params (OverlappedComponent :type Primitive%20Component%20Object%20Reference) (OtherActor :type Actor%20Object%20Reference) (OtherComp :type Primitive%20Component%20Object%20Reference) (OtherBodyIndex :type Integer) (bFromSweep :type Boolean) (SweepResult :type Hit%20Result%20Structure%20%28by%20ref%29))
  (Variables|Default|SetTouchingWall true)
  (Variables|Default|SetTouchingWallLocation (Transformation|GetActorLocation OtherActor))
  (Math|Integer|IncrementInt (Variables|Default|GetWallTouch)))

(event OnComponentEndOverlap(CapsuleComponent)
  (params (OverlappedComponent :type Primitive%20Component%20Object%20Reference) (OtherActor :type Actor%20Object%20Reference) (OtherComp :type Primitive%20Component%20Object%20Reference) (OtherBodyIndex :type Integer))
  (Variables|Default|SetTouchingWall false))

(event EventBeginPlay
  (|CallParentFunction)
  (bind _returnvalue (Actor|GetActorOfClass "/Game/Blueprints/AStarBPs/BP_AStarMapGen.BP_AStarMapGen_C"))
  (bind _output_get (Variables|Default|SetGridRef _returnvalue))
  (Variables|Default|SetWalls (Class|AStarMapGeneration|GetWallSpaces _output_get))
  (bind _outactors (Actor|GetAllActorswithTag "AStarManager"))
  (for _array_element _outactors
    (Utilities|IsValid (Actor|GetComponentbyClass _array_element "/Script/LearningAgents.LearningAgentsManager")
      (:Is%20Valid
        (Class|LearningAgentsManager|AddAgent (Actor|GetComponentbyClass _array_element "/Script/LearningAgents.LearningAgentsManager") self)
        (Variables|Default|SetFoundManager? true))))
  (if (not (Variables|Default|GetFoundManager?))
    (Development|PrintString "Could not find Learning Agents manager. Did we forget to add one to the scene?")))

(fn ConstructionScript)

(fn ResettoNewStartLocation
  (while (LocalVariables|GetInvalidTransform)
    (LocalVariables|SetCandidateTransform (Math|Transform|MakeTransform "100.000000,100.000000,0.000000"))
    (LocalVariables|SetInvalidTransform false)
    (bind _outactors (Actor|GetAllActorsOfClass "/Game/Blueprints/AStarBPs/BP_AStarPawn.BP_AStarPawn_C"))
    (for _array_element _outactors
      (if (not (LocalVariables|GetInvalidTransform))
        (if (< (Math|Vector|Distance(Vector) (Transformation|GetActorLocation _array_element) (.location (LocalVariables|GetCandidateTransform))) 2e+02)
          (LocalVariables|SetInvalidTransform false)))))
  (Transformation|SetActorTransform (LocalVariables|GetCandidateTransform) false true)
  (Variables|Default|SetWallTouch 0))

(fn Raycast
  (params (Angles :type Array%20of%20Floats%20%28double-precision%29) (Ray%20Length :type Float%20%28double-precision%29))
  (bind _returnvalue (Transformation|GetActorLocation))
  (Utilities|Array|Clear (LocalVariables|GetWallPos))
  (for _index (range 0 7)
    (bind (_outhit _returnvalue_2) (Collision|LineTraceByChannel _returnvalue (+ (* (Math|Vector|GetForwardVector (Math|Rotator|MakeRotator 0.0 0.0 (Math|Conversions|ToFloat(Integer) (* _index 45)))) Ray%20Length) _returnvalue) "TraceTypeQuery1" false 0 "None"))
    (if _returnvalue_2
      (Utilities|Array|Add (LocalVariables|GetWallPos) (.Location (Collision|BreakHitResult _outhit)))
      (else
        (Utilities|Array|Add :TargetArray (LocalVariables|GetWallPos)))))
  (return (LocalVariables|GetWallPos)))