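; Learning Agents training environment that teaches BP_AStarPawn agents to reach a target location while avoiding walls.
; Reward combines distance progress since the last location, a small step penalty, tiered proximity and arrival bonuses, and a wall-proximity penalty found by looping over the pawn's Walls with debug prints.
; Episodes end only by truncation on reaching the target, and reset calls the pawn's ResetToNewStartLocation.
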(fn GatherAgentReward
  (params (AgentId :type Integer))
  (LocalVariables|SetRewardActor (Class|LearningAgentsManagerListener|GetAgent AgentId "/Game/Blueprints/BP_AStarPawn.BP_AStarPawn_C"))
  (bind _array_element (Utilities|Array|ForEachLoopwithBreak (Variables|/Game/Blueprints/BP_AStarPawn.BP_AStarPawn_C|GetWalls (LocalVariables|GetRewardActor)) :!label _label)
    (:LoopBody
      (Development|PrintString 0 (Utilities|String|ToString(Float) (Class|LearningAgentsRewards|MakeRewardonCondition (Utilities|Operators|EqualEqual (Pawn|GetNavAgentLocation (LocalVariables|GetRewardActor)) (Math|Conversions|ToVector(Vector2D) _array_element 5e+01) 6e+01) -1.0 "ConditionReward" false 0)))
      (if (Utilities|Operators|EqualEqual (Pawn|GetNavAgentLocation (LocalVariables|GetRewardActor)) (Math|Conversions|ToVector(Vector2D) _array_element 5e+01) 6e+01)
        (goto _label Break)))
    (:Completed
      (return (+ (Class|LearningAgentsRewards|MakeReward (- (Math|Vector|Distance2D(Vector) (Variables|/Game/Blueprints/BP_AStarPawn.BP_AStarPawn_C|GetLastLocation (LocalVariables|GetRewardActor)) (Variables|/Game/Blueprints/BP_AStarPawn.BP_AStarPawn_C|GetTargetLocation (LocalVariables|GetRewardActor))) (Math|Vector|Distance2D(Vector) (Pawn|GetNavAgentLocation (LocalVariables|GetRewardActor)) (Variables|/Game/Blueprints/BP_AStarPawn.BP_AStarPawn_C|GetTargetLocation (LocalVariables|GetRewardActor)))) 0.01 "Reward" false 0) (Class|LearningAgentsRewards|MakeReward -0.001 1.0 "Reward" false 0) (Class|LearningAgentsRewards|MakeRewardonLocationDifferenceBelowThreshold (Pawn|GetNavAgentLocation (LocalVariables|GetRewardActor)) (Variables|/Game/Blueprints/BP_AStarPawn.BP_AStarPawn_C|GetTargetLocation (LocalVariables|GetRewardActor)) 5e+02 1.0 "LocationDifferenceBelowThresholdReward" false 0) (Class|LearningAgentsRewards|MakeRewardonCondition (Utilities|Operators|EqualEqual (Pawn|GetNavAgentLocation (LocalVariables|GetRewardActor)) (Variables|/Game/Blueprints/BP_AStarPawn.BP_AStarPawn_C|GetTargetLocation (LocalVariables|GetRewardActor)) 1e+02) 1e+01 "ConditionReward" false 0) (Class|LearningAgentsRewards|MakeRewardonCondition (Utilities|Operators|EqualEqual (Pawn|GetNavAgentLocation (LocalVariables|GetRewardActor)) (Math|Conversions|ToVector(Vector2D) _array_element 5e+01) 6e+01) -1.0 "ConditionReward" false 0) (Class|LearningAgentsRewards|MakeRewardonLocationDifferenceBelowThreshold (Pawn|GetNavAgentLocation (LocalVariables|GetRewardActor)) (Variables|/Game/Blueprints/BP_AStarPawn.BP_AStarPawn_C|GetTargetLocation (LocalVariables|GetRewardActor)) 2.5e+02 5.0 "LocationDifferenceBelowThresholdReward" false 0) (Class|LearningAgentsRewards|MakeRewardonLocationDifferenceBelowThreshold (Pawn|GetNavAgentLocation (LocalVariables|GetRewardActor)) (Variables|/Game/Blueprints/BP_AStarPawn.BP_AStarPawn_C|GetTargetLocation (LocalVariables|GetRewardActor)) 1.5e+02 7.5 "LocationDifferenceBelowThresholdReward" false 0))))))

(fn GatherAgentCompletion
  (params (AgentId :type Integer))
  (bind _returnvalue (Class|LearningAgentsManagerListener|GetAgent AgentId "/Game/Blueprints/BP_AStarPawn.BP_AStarPawn_C"))
  (return (Class|LearningAgentsCompletions|MakeCompletiononCondition (Utilities|Operators|EqualEqual (Transformation|GetActorLocation _returnvalue) (Variables|/Game/Blueprints/BP_AStarPawn.BP_AStarPawn_C|GetTargetLocation _returnvalue) 1e+02) "Truncation" "ConditionCompletion" true 0)))

(fn ResetAgentEpisode
  (params (AgentId :type Integer))
  (Default|ResettoNewStartLocation (Class|LearningAgentsManagerListener|GetAgent AgentId "/Game/Blueprints/BP_AStarPawn.BP_AStarPawn_C")))