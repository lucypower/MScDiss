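; Learning Agents interactor that lets a policy stock and price a shop on BP_FSMPawn2 based on player stats.
; Observes weapon class, normalized gold and reputation, and per-item discount states.
; Each action advances a fixed state machine through evaluation, reset, item pricing, discounting and display, applying policy outputs only in the deciding states.
; Prices scale with player gold; a random roll against learned chance can then raise, keep or cut each.
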(fn SpecifyAgentObservation
  (params (InObservationSchema :type Learning%20Agents%20Observation%20Schema%20Object%20Reference))
  (return (Class|LearningAgentsObservations|SpecifyStructObservation InObservationSchema (Utilities|Map|MakeMap "WeaponClass" (Class|LearningAgentsObservations|SpecifyFloatObservation InObservationSchema 1.0) "CurrentGold" (Class|LearningAgentsObservations|SpecifyFloatObservation InObservationSchema 1.0) "Reputation" (Class|LearningAgentsObservations|SpecifyFloatObservation InObservationSchema 1.0) "DiscountApplied" (Class|LearningAgentsObservations|SpecifyArrayObservation InObservationSchema (Class|LearningAgentsObservations|SpecifyFloatObservation InObservationSchema 1.0) 3)))))

(fn GatherAgentObservation
  (params (InObservationObject :type Learning%20Agents%20Observation%20Object%20Object%20Reference) (AgentId :type Integer))
  (LocalVariables|SetObsActor (Class|LearningAgentsManagerListener|GetAgent AgentId "/Game/Blueprints/FSMBPs/BP_FSMPawn2.BP_FSMPawn2_C"))
  (Utilities|FlowControl|Sequence
    (:then_0
      (Utilities|Array|Clear (LocalVariables|GetDiscountFloats))
      (for _array_element (Variables|/Game/Blueprints/FSMBPs/BP_FSMPawn2.BP_FSMPawn2_C|GetDiscountApplied (LocalVariables|GetObsActor))
        (Utilities|Array|Add (LocalVariables|GetDiscountFloats) (Class|LearningAgentsObservations|MakeFloatObservation InObservationObject (Math|Float|NormalizetoRange _array_element 0.0 3.0) "FloatObservation" false 0))))
    (:then_1
      (return (Class|LearningAgentsObservations|MakeStructObservation InObservationObject (Utilities|Map|MakeMap "WeaponClass" (Class|LearningAgentsObservations|MakeFloatObservation InObservationObject (Math|Conversions|ToFloat(Integer) (Variables|/Game/Blueprints/FSMBPs/BP_FSMPawn2.BP_FSMPawn2_C|GetPlayerWeaponClass (LocalVariables|GetObsActor))) "FloatObservation" false 0) "CurrentGold" (Class|LearningAgentsObservations|MakeFloatObservation InObservationObject (Math|Float|NormalizetoRange (Math|Conversions|ToFloat(Integer) (Variables|/Game/Blueprints/FSMBPs/BP_FSMPawn2.BP_FSMPawn2_C|GetPlayerCurrentGold (LocalVariables|GetObsActor))) 0.0 1e+03) "FloatObservation" false 0) "Reputation" (Class|LearningAgentsObservations|MakeFloatObservation InObservationObject (Math|Float|NormalizetoRange (Math|Conversions|ToFloat(Integer) (Variables|/Game/Blueprints/FSMBPs/BP_FSMPawn2.BP_FSMPawn2_C|GetPlayerReputation (LocalVariables|GetObsActor))) 0.0 1e+01) "FloatObservation" false 0) "DiscountApplied" (Class|LearningAgentsObservations|MakeArrayObservation InObservationObject (LocalVariables|GetDiscountFloats) 3)))))))

(fn SpecifyAgentAction
  (params (InActionSchema :type Learning%20Agents%20Action%20Schema%20Object%20Reference))
  (return (Class|LearningAgentsActions|SpecifyStructAction InActionSchema (Utilities|Map|MakeMap "ItemName0" (Class|LearningAgentsActions|SpecifyFloatAction InActionSchema 1.0 "ItemName0") "ItemPrice0" (Class|LearningAgentsActions|SpecifyFloatAction InActionSchema 1.0 "ItemPrice0") "ItemName1" (Class|LearningAgentsActions|SpecifyFloatAction InActionSchema 1.0 "ItemName1") "ItemPrice1" (Class|LearningAgentsActions|SpecifyFloatAction InActionSchema 1.0 "ItemPrice1") "ItemName2" (Class|LearningAgentsActions|SpecifyFloatAction InActionSchema 1.0 "ItemName2") "ItemPrice2" (Class|LearningAgentsActions|SpecifyFloatAction InActionSchema 1.0 "ItemPrice2") "DiscountChance" (Class|LearningAgentsActions|SpecifyFloatAction InActionSchema 1.0 "Discount") "DiscountMultiplier" (Class|LearningAgentsActions|SpecifyFloatAction InActionSchema 1.0 "Discount")))))

(fn PerformAgentAction
  (params (InActionObject :type Learning%20Agents%20Action%20Object%20Object%20Reference) (InActionObjectElement :type Learning%20Agents%20Action%20Object%20Element%20Structure%20%28by%20ref%29) (AgentId :type Integer))
  (LocalVariables|SetActActor (Class|LearningAgentsManagerListener|GetAgent AgentId "/Game/Blueprints/FSMBPs/BP_FSMPawn2.BP_FSMPawn2_C"))
  (switch Utilities|FlowControl|Switch|SwitchonFSMState (Variables|/Game/Blueprints/FSMBPs/BP_FSMPawn2.BP_FSMPawn2_C|GetFSMState (LocalVariables|GetActActor))
    (:NewEnumerator1
      (Variables|/Game/Blueprints/FSMBPs/BP_FSMPawn2.BP_FSMPawn2_C|SetFSMState (LocalVariables|GetActActor) "NewEnumerator7"))
    (:NewEnumerator2
      (Variables|/Game/Blueprints/FSMBPs/BP_FSMPawn2.BP_FSMPawn2_C|SetFSMState (LocalVariables|GetActActor) "NewEnumerator4"))
    (:NewEnumerator7
      (Variables|/Game/Blueprints/FSMBPs/BP_FSMPawn2.BP_FSMPawn2_C|SetFSMState (LocalVariables|GetActActor) "NewEnumerator2"))
    (:NewEnumerator4
      (Variables|/Game/Blueprints/FSMBPs/BP_FSMPawn2.BP_FSMPawn2_C|SetFSMState (LocalVariables|GetActActor) "NewEnumerator5"))
    (:NewEnumerator5
      (Variables|/Game/Blueprints/FSMBPs/BP_FSMPawn2.BP_FSMPawn2_C|SetFSMState (LocalVariables|GetActActor) "NewEnumerator6"))
    (:NewEnumerator6
      (Variables|/Game/Blueprints/FSMBPs/BP_FSMPawn2.BP_FSMPawn2_C|SetFSMState (LocalVariables|GetActActor) "NewEnumerator1")))
  (switch Utilities|FlowControl|Switch|SwitchonFSMState (Variables|/Game/Blueprints/FSMBPs/BP_FSMPawn2.BP_FSMPawn2_C|GetFSMState (LocalVariables|GetActActor))
    (:NewEnumerator2
      ;[0.15 0.15 0.15 0.5] ResetShop
      (if (Utilities|Array|IsNotEmpty (Variables|/Game/Blueprints/FSMBPs/BP_FSMPawn2.BP_FSMPawn2_C|GetShopItemNames (LocalVariables|GetActActor)))
        (Utilities|Array|Clear (Variables|/Game/Blueprints/FSMBPs/BP_FSMPawn2.BP_FSMPawn2_C|GetShopItemNames (LocalVariables|GetActActor)))
        (Utilities|Array|Clear (Variables|/Game/Blueprints/FSMBPs/BP_FSMPawn2.BP_FSMPawn2_C|GetShopItemPrices (LocalVariables|GetActActor))))
      (Variables|/Game/Blueprints/FSMBPs/BP_FSMPawn2.BP_FSMPawn2_C|SetShopText (LocalVariables|GetActActor) "")
      (Variables|/Game/Blueprints/FSMBPs/BP_FSMPawn2.BP_FSMPawn2_C|SetAppliedDiscount? (LocalVariables|GetActActor) false))
    (:NewEnumerator7
      ;[0.15 0.15 0.15 0.5] Get Player Stats
      (Variables|/Game/Blueprints/FSMBPs/BP_FSMPawn2.BP_FSMPawn2_C|SetPlayerWeaponClass (LocalVariables|GetActActor) (Variables|/Script/MScDiss.FSMPlayerPawnComponent|GetWeaponClass (Variables|Default|GetPlayer)))
      (Variables|/Game/Blueprints/FSMBPs/BP_FSMPawn2.BP_FSMPawn2_C|SetPlayerCurrentGold (LocalVariables|GetActActor) (Variables|/Script/MScDiss.FSMPlayerPawnComponent|GetCurrentGold (Variables|Default|GetPlayer)))
      (Variables|/Game/Blueprints/FSMBPs/BP_FSMPawn2.BP_FSMPawn2_C|SetPlayerReputation (LocalVariables|GetActActor) (Variables|/Script/MScDiss.FSMPlayerPawnComponent|GetReputation (Variables|Default|GetPlayer))))
    (:NewEnumerator4
      ;[0.15 0.15 0.15 0.5] Deciding Items and Prices
      (bind _outelements (Class|LearningAgentsActions|GetStructAction InActionObject InActionObjectElement))
      (bind _outvalue (Class|LearningAgentsActions|GetFloatAction InActionObject (.Value (Utilities|Map|Find _outelements "ItemName0")) "ItemName0" false 0))
      (if (> (Math|Float|Clamp(Float) _outvalue) 0.5)
        (Variables|/Game/Blueprints/FSMBPs/BP_FSMPawn2.BP_FSMPawn2_C|SetSelectedWeaponIndex (LocalVariables|GetActActor) 1)
        (Utilities|Array|Add (Variables|/Game/Blueprints/FSMBPs/BP_FSMPawn2.BP_FSMPawn2_C|GetShopItemNames (LocalVariables|GetActActor)) (Utilities|Array|Get(acopy) (Variables|/Game/Blueprints/FSMBPs/BP_FSMPawn2.BP_FSMPawn2_C|GetWeaponNames (LocalVariables|GetActActor)) 1))
        (else
          (Variables|/Game/Blueprints/FSMBPs/BP_FSMPawn2.BP_FSMPawn2_C|SetSelectedWeaponIndex (LocalVariables|GetActActor) 0)
          (Utilities|Array|Add (Variables|/Game/Blueprints/FSMBPs/BP_FSMPawn2.BP_FSMPawn2_C|GetShopItemNames (LocalVariables|GetActActor)) (Utilities|Array|Get(acopy) (Variables|/Game/Blueprints/FSMBPs/BP_FSMPawn2.BP_FSMPawn2_C|GetWeaponNames (LocalVariables|GetActActor))))))
      (bind _outvalue_2 (Class|LearningAgentsActions|GetFloatAction InActionObject (.Value (Utilities|Map|Find _outelements "ItemName1")) "ItemName1" false 0))
      (Utilities|Array|Add (Variables|/Game/Blueprints/FSMBPs/BP_FSMPawn2.BP_FSMPawn2_C|GetShopItemNames (LocalVariables|GetActActor)) (Utilities|Array|Get(acopy) (Variables|/Game/Blueprints/FSMBPs/BP_FSMPawn2.BP_FSMPawn2_C|GetItemNames (LocalVariables|GetActActor)) (Math|Float|Round (Math|Float|Clamp(Float) (* _outvalue_2 1.2) 0.0 2.0))))
      (bind _outvalue_3 (Class|LearningAgentsActions|GetFloatAction InActionObject (.Value (Utilities|Map|Find _outelements "ItemName2")) "ItemName2" false 0))
      (Utilities|Array|Add (Variables|/Game/Blueprints/FSMBPs/BP_FSMPawn2.BP_FSMPawn2_C|GetShopItemNames (LocalVariables|GetActActor)) (Utilities|Array|Get(acopy) (Variables|/Game/Blueprints/FSMBPs/BP_FSMPawn2.BP_FSMPawn2_C|GetItemNames (LocalVariables|GetActActor)) (Math|Float|Round (Math|Float|Clamp(Float) (* _outvalue_3 1.2) 0.0 2.0))))
      (bind _outvalue_4 (Class|LearningAgentsActions|GetFloatAction InActionObject (.Value (Utilities|Map|Find _outelements "ItemPrice0")) "ItemPrice0" false 0))
      (Utilities|Array|Add (Variables|/Game/Blueprints/FSMBPs/BP_FSMPawn2.BP_FSMPawn2_C|GetShopItemPrices (LocalVariables|GetActActor)) (Math|Float|Round (* (Variables|/Script/MScDiss.FSMPlayerPawnComponent|GetCurrentGold (Variables|Default|GetPlayer)) (Math|Float|MapRangeClamped _outvalue_4 0.0 1.0 0.2 1.5))))
      (bind _outvalue_5 (Class|LearningAgentsActions|GetFloatAction InActionObject (.Value (Utilities|Map|Find _outelements "ItemPrice1")) "ItemPrice1" false 0))
      (Utilities|Array|Add (Variables|/Game/Blueprints/FSMBPs/BP_FSMPawn2.BP_FSMPawn2_C|GetShopItemPrices (LocalVariables|GetActActor)) (Math|Float|Round (* (Variables|/Script/MScDiss.FSMPlayerPawnComponent|GetCurrentGold (Variables|Default|GetPlayer)) (Math|Float|MapRangeClamped _outvalue_5 0.0 1.0 0.2 0.8))))
      (bind _outvalue_6 (Class|LearningAgentsActions|GetFloatAction InActionObject (.Value (Utilities|Map|Find _outelements "ItemPrice2")) "ItemPrice2" false 0))
      (Utilities|Array|Add (Variables|/Game/Blueprints/FSMBPs/BP_FSMPawn2.BP_FSMPawn2_C|GetShopItemPrices (LocalVariables|GetActActor)) (Math|Float|Round (* (Variables|/Script/MScDiss.FSMPlayerPawnComponent|GetCurrentGold (Variables|Default|GetPlayer)) (Math|Float|MapRangeClamped _outvalue_6 0.0 1.0 0.2 0.7)))))
    (:NewEnumerator5
      ;[0.15 0.15 0.15 0.5] Decide Discount
      (bind _outelements_2 (Class|LearningAgentsActions|GetStructAction InActionObject InActionObjectElement))
      (for _index (range 0 2)
        (bind _outvalue_7 (Class|LearningAgentsActions|GetFloatAction InActionObject (.Value (Utilities|Map|Find _outelements_2 "DiscountChance")) "FloatAction" false 0))
        (if (> (Math|Float|MapRangeClamped _outvalue_7 -1.0 1.0 0.0 1.0) (Math|Random|RandomFloatinRange 0.0 1.0))
          (bind _outvalue_8 (Class|LearningAgentsActions|GetFloatAction InActionObject (.Value (Utilities|Map|Find _outelements_2 "DiscountMultiplier")) "FloatAction" false 0))
          (Utilities|Array|SetArrayElem (Variables|/Game/Blueprints/FSMBPs/BP_FSMPawn2.BP_FSMPawn2_C|GetShopItemPrices (LocalVariables|GetActActor)) _index (* (Utilities|Array|Get(acopy) (Variables|/Game/Blueprints/FSMBPs/BP_FSMPawn2.BP_FSMPawn2_C|GetShopItemPrices (LocalVariables|GetActActor)) _index) (Utilities|Select :Index (Math|Float|Round (Math|Float|Clamp(Float) _outvalue_8 0.0 2.0)) :Option%200 (Math|Float|MakeLiteralFloat 1.8) :Option%201 (Math|Float|MakeLiteralFloat 1.0) :Option%202 (Math|Float|MakeLiteralFloat 0.2))))
          (Utilities|Array|SetArrayElem (Variables|/Game/Blueprints/FSMBPs/BP_FSMPawn2.BP_FSMPawn2_C|GetDiscountApplied (LocalVariables|GetActActor)) _index (Math|Conversions|ToFloat(Integer) (Math|Float|Round (Math|Float|Clamp(Float) _outvalue_8 0.0 2.0))))
          (else
            (Utilities|Array|SetArrayElem (Variables|/Game/Blueprints/FSMBPs/BP_FSMPawn2.BP_FSMPawn2_C|GetDiscountApplied (LocalVariables|GetActActor)) _index 3.0)))))
    (:NewEnumerator6
      (Variables|/Game/Blueprints/FSMBPs/BP_FSMPawn2.BP_FSMPawn2_C|SetProcessComplete? (LocalVariables|GetActActor) true))))