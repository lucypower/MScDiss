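; Manager actor that sets up Learning Agents training or inference for BP_FSMPawn2 actors, with BP_MLShop widgets for the first three.
; BeginPlay builds the interactor, policy, critic, training environment and shared-memory PPO trainer, feeding the player pawn's component to interactor and environment.
; RunInference keeps saved networks, respawns the player pawn and times policy inference until the first pawn completes.
; Otherwise, networks reinitialize and Tick trains, ahead of the pawns via tick prerequisites.
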(event EventTick
  (params (DeltaSeconds :type Float%20%28single-precision%29))
  (if (Variables|Default|GetRun%20Inference)
    (if (not (Variables|/Game/Blueprints/FSMBPs/BP_FSMPawn2.BP_FSMPawn2_C|GetProcessComplete? (Utilities|Array|Get(acopy) (Variables|Default|GetFSMActors))))
      (Utilities|FlowControl|Sequence
        (:then_0
          (Variables|Default|SetInferenceStartTime (Class|InferenceTiming|GetInferenceTime)))
        (:then_1
          (Class|LearningAgentsPolicy|RunInference (Variables|Default|GetPolicy) 0.0))
        (:then_2
          (Variables|Default|SetTotalInferenceTime (+ (Variables|Default|GetTotalInferenceTime) (- (Class|InferenceTiming|GetInferenceTime) (Variables|Default|GetInferenceStartTime)))))))
    (else
      (Class|LearningAgentsPPOTrainer|RunTraining (Variables|Default|GetPPOTrainer) (Variables|Default|GetTrainer%20Training%20Settings) (Variables|Default|GetTraining%20Game%20Settings) true true))))

(event EventBeginPlay
  (bind _shared_memory_settings (Variables|Default|GetShared%20Memory%20Settings))
  (bind _run_inference (Variables|Default|GetRun%20Inference))
  (bind _returnvalue (not _run_inference))
  (Utilities|FlowControl|Sequence
    (:then_0
      (bind _outactors (Actor|GetAllActorsOfClass "/Game/Blueprints/FSMBPs/BP_FSMPawn2.BP_FSMPawn2_C"))
      (bind _output_get (Variables|Default|SetFSMActors _outactors))
      (Actor|Tick|AddTickPrerequisiteActor _output_get self))
    (:then_1
      (bind _returnvalue_2 (UserInterface|CreateWidget "/Game/Blueprints/FSMBPs/BP_MLShop.BP_MLShop_C" 0 (Utilities|Array|Get(acopy) (Variables|Default|GetFSMActors))))
      (UserInterface|Viewport|AddtoViewport _returnvalue_2 0)
      (Class|UserWidget|SetPositioninViewport _returnvalue_2 "(X=100.000000,Y=500.000000)" true)
      (bind _returnvalue_3 (UserInterface|CreateWidget "/Game/Blueprints/FSMBPs/BP_MLShop.BP_MLShop_C" 0 (Utilities|Array|Get(acopy) (Variables|Default|GetFSMActors) 1)))
      (UserInterface|Viewport|AddtoViewport _returnvalue_3 0)
      (Class|UserWidget|SetPositioninViewport _returnvalue_3 "(X=600.000000,Y=500.000000)" true)
      (bind _returnvalue_4 (UserInterface|CreateWidget "/Game/Blueprints/FSMBPs/BP_MLShop.BP_MLShop_C" 0 (Utilities|Array|Get(acopy) (Variables|Default|GetFSMActors) 2)))
      (UserInterface|Viewport|AddtoViewport _returnvalue_4 0)
      (Class|UserWidget|SetPositioninViewport _returnvalue_4 "(X=1100.000000,Y=500.000000)" true))
    (:then_2
      (bind _returnvalue_5 (Actor|GetActorOfClass "/Game/Blueprints/FSMBPs/BP_FSMPlayerPawn.BP_FSMPlayerPawn_C"))
      (Variables|Default|SetPlayer _returnvalue_5))
    (:then_3
      (bind _returnvalue_6 (Class|LearningAgentsInteractor|MakeInteractor (Variables|Default|GetLearningAgentsManager) "/Game/Blueprints/Learning/FSM2/BP_FSMInteractor2.BP_FSMInteractor2_C" "Interactor"))
      (bind _output_get_2 (Variables|Default|SetInteractor _returnvalue_6))
      (Variables|/Game/Blueprints/Learning/FSM2/BP_FSMInteractor2.BP_FSMInteractor2_C|SetPlayer _output_get_2 (Actor|GetComponentbyClass (Variables|Default|GetPlayer) "/Script/MScDiss.FSMPlayerPawnComponent")))
    (:then_4
      (bind _returnvalue_7 (Class|LearningAgentsPolicy|MakePolicy (Variables|Default|GetLearningAgentsManager) (Variables|Default|GetInteractor) "/Script/LearningAgents.LearningAgentsPolicy" "FSMPolicy" "/Game/Blueprints/Learning/FSM2/DA_FSMEncoder2.DA_FSMEncoder2" "/Game/Blueprints/Learning/FSM2/DA_FSMPolicy2.DA_FSMPolicy2" "/Game/Blueprints/Learning/FSM2/DA_FSMDecoder2.DA_FSMDecoder2" _returnvalue _returnvalue _returnvalue (Variables|Default|GetPolicy%20Settings) 1234))
      (Variables|Default|SetPolicy _returnvalue_7))
    (:then_5
      (bind _returnvalue_8 (Class|LearningAgentsCritic|MakeCritic (Variables|Default|GetLearningAgentsManager) (Variables|Default|GetInteractor) (Variables|Default|GetPolicy) "/Script/LearningAgents.LearningAgentsCritic" "FSMCritic" "/Game/Blueprints/Learning/FSM2/DA_FSMCritic2.DA_FSMCritic2" (not (Variables|Default|GetRun%20Inference)) (Variables|Default|GetCritic%20Settings) 1234))
      (Variables|Default|SetCritic _returnvalue_8))
    (:then_6
      (bind _returnvalue_9 (Class|LearningAgentsTrainingEnvironment|MakeTrainingEnvironment (Variables|Default|GetLearningAgentsManager) "/Game/Blueprints/Learning/FSM2/BP_FSMTrainingEnv2.BP_FSMTrainingEnv2_C" "TrainingEnvironment"))
      (bind _output_get_3 (Variables|Default|SetTrainingEnv _returnvalue_9))
      (Variables|/Game/Blueprints/Learning/FSM2/BP_FSMTrainingEnv2.BP_FSMTrainingEnv2_C|SetPlayer _output_get_3 (Actor|GetComponentbyClass (Variables|Default|GetPlayer) "/Script/MScDiss.FSMPlayerPawnComponent")))
    (:then_7
      (bind _returnvalue_10 (Class|LearningAgentsCommunicatorLibrary|SpawnSharedMemoryTrainingProcess (Variables|Default|GetTrainer%20Process%20Settings) _shared_memory_settings))
      (bind _returnvalue_11 (Class|LearningAgentsCommunicatorLibrary|MakeSharedMemoryCommunicator _returnvalue_10 _shared_memory_settings))
      (Variables|Default|SetCommunicator _returnvalue_11))
    (:then_8
      (bind _returnvalue_12 (Class|LearningAgentsPPOTrainer|MakePPOTrainer (Variables|Default|GetLearningAgentsManager) (Variables|Default|GetInteractor) (Variables|Default|GetTrainingEnv) (Variables|Default|GetPolicy) (Variables|Default|GetCritic) (Variables|Default|GetCommunicator) "/Script/LearningAgentsTraining.LearningAgentsPPOTrainer" "PPOTrainer" (Variables|Default|GetTrainer%20Settings)))
      (Variables|Default|SetPPOTrainer _returnvalue_12))
    (:then_9
      (if (Variables|Default|GetRun%20Inference)
        (Default|RespawnPlayerPawn (Variables|Default|GetFSMActors))))))

(fn ConstructionScript)