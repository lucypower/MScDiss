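; Learning Agents interactor that lets a trained agent drive a BP_FSMPawn shopkeeper state machine, stocking and pricing a shop for the player.
; Observations combine player weapon class, gold and reputation with step-completion flags and the current FSM state.
; Each action picks the next state, which resets the shop, reads player stats, selects items and prices, applies discounts or completes the process.
; Float outputs map to item indices and prices, with random price scaling and randomly chosen discounted items.
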(fn SpecifyAgentObservation
  (params (InObservationSchema :type Learning%20Agents%20Observation%20Schema%20Object%20Reference))
  (return (Class|LearningAgentsObservations|SpecifyStructObservation InObservationSchema (Utilities|Map|MakeMap "PlayerStats" (Class|LearningAgentsObservations|SpecifyStructObservation InObservationSchema (Utilities|Map|MakeMap "WeaponClass" (Class|LearningAgentsObservations|SpecifyFloatObservation InObservationSchema 1.0) "CurrentGold" (Class|LearningAgentsObservations|SpecifyFloatObservation InObservationSchema 1.0) "Reputation" (Class|LearningAgentsObservations|SpecifyFloatObservation InObservationSchema 1.0))) "bStatesCompleted" (Class|LearningAgentsObservations|SpecifyStructObservation InObservationSchema (Utilities|Map|MakeMap "ResetShop" (Class|LearningAgentsObservations|SpecifyBoolObservation InObservationSchema) "PlayerObserved" (Class|LearningAgentsObservations|SpecifyBoolObservation InObservationSchema) "DecideItems" (Class|LearningAgentsObservations|SpecifyBoolObservation InObservationSchema) "DecideDiscount" (Class|LearningAgentsObservations|SpecifyBoolObservation InObservationSchema) "ProcessComplete" (Class|LearningAgentsObservations|SpecifyBoolObservation InObservationSchema))) "CurrentState" (Class|LearningAgentsObservations|SpecifyEnumObservation InObservationSchema "/Game/Blueprints/FSMBPs/FSMState.FSMState")))))

(fn GatherAgentObservation
  (params (InObservationObject :type Learning%20Agents%20Observation%20Object%20Object%20Reference) (AgentId :type Integer))
  (LocalVariables|SetObsActor (Class|LearningAgentsManagerListener|GetAgent AgentId "/Game/Blueprints/FSMBPs/BP_FSMPawn.BP_FSMPawn_C"))
  (return (Class|LearningAgentsObservations|MakeStructObservation InObservationObject (Utilities|Map|MakeMap "PlayerStats" (Class|LearningAgentsObservations|MakeStructObservation InObservationObject (Utilities|Map|MakeMap "WeaponClass" (Class|LearningAgentsObservations|MakeFloatObservation InObservationObject (Math|Conversions|ToFloat(Integer) (Variables|/Script/MScDiss.FSMPlayerPawnComponent|GetWeaponClass (Variables|Default|GetPlayer))) "FloatObservation" false 0) "CurrentGold" (Class|LearningAgentsObservations|MakeFloatObservation InObservationObject (Math|Conversions|ToFloat(Integer) (Variables|/Script/MScDiss.FSMPlayerPawnComponent|GetCurrentGold (Variables|Default|GetPlayer))) "FloatObservation" false 0) "Reputation" (Class|LearningAgentsObservations|MakeFloatObservation InObservationObject (Math|Conversions|ToFloat(Integer) (Variables|/Script/MScDiss.FSMPlayerPawnComponent|GetReputation (Variables|Default|GetPlayer))) "FloatObservation" false 0))) "bStatesCompleted" (Class|LearningAgentsObservations|MakeStructObservation InObservationObject (Utilities|Map|MakeMap "ResetShop" (Class|LearningAgentsObservations|MakeBoolObservation InObservationObject (Variables|/Game/Blueprints/FSMBPs/BP_FSMPawn.BP_FSMPawn_C|GetResetShop? (LocalVariables|GetObsActor)) "BoolObservation" false 0) "PlayerObserved" (Class|LearningAgentsObservations|MakeBoolObservation InObservationObject (Variables|/Game/Blueprints/FSMBPs/BP_FSMPawn.BP_FSMPawn_C|GetObservedPlayer? (LocalVariables|GetObsActor)) "BoolObservation" false 0) "DecideItems" (Class|LearningAgentsObservations|MakeBoolObservation InObservationObject (Variables|/Game/Blueprints/FSMBPs/BP_FSMPawn.BP_FSMPawn_C|GetDecideItems? (LocalVariables|GetObsActor)) "BoolObservation" false 0) "DecideDiscount" (Class|LearningAgentsObservations|MakeBoolObservation InObservationObject (Variables|/Game/Blueprints/FSMBPs/BP_FSMPawn.BP_FSMPawn_C|GetDecideDiscount? (LocalVariables|GetObsActor)) "BoolObservation" false 0) "ProcessComplete" (Class|LearningAgentsObservations|MakeBoolObservation InObservationObject (Variables|/Game/Blueprints/FSMBPs/BP_FSMPawn.BP_FSMPawn_C|GetProcessComplete? (LocalVariables|GetObsActor)) "BoolObservation" false 0))) "CurrentState" (Class|LearningAgentsObservations|MakeEnumObservation InObservationObject "/Game/Blueprints/FSMBPs/FSMState.FSMState" (Variables|/Game/Blueprints/FSMBPs/BP_FSMPawn.BP_FSMPawn_C|GetFSMState (LocalVariables|GetObsActor)) "EnumObservation" false 0)))))

(fn SpecifyAgentAction
  (params (InActionSchema :type Learning%20Agents%20Action%20Schema%20Object%20Reference))
  (return (Class|LearningAgentsActions|SpecifyStructAction InActionSchema (Utilities|Map|MakeMap "ItemName0" (Class|LearningAgentsActions|SpecifyFloatAction InActionSchema 1.0 "ItemName0") "ItemPrice0" (Class|LearningAgentsActions|SpecifyFloatAction InActionSchema 1.0 "ItemPrice0") "ItemName1" (Class|LearningAgentsActions|SpecifyFloatAction InActionSchema 1.0 "ItemName1") "ItemPrice1" (Class|LearningAgentsActions|SpecifyFloatAction InActionSchema 1.0 "ItemPrice1") "ItemName2" (Class|LearningAgentsActions|SpecifyFloatAction InActionSchema 1.0 "ItemName2") "ItemPrice2" (Class|LearningAgentsActions|SpecifyFloatAction InActionSchema 1.0 "ItemPrice2") "ChangeState" (Class|LearningAgentsActions|SpecifyEnumAction InActionSchema "/Game/Blueprints/FSMBPs/FSMState.FSMState" 0 "ChangeState") "Discount" (Class|LearningAgentsActions|SpecifyFloatAction InActionSchema 1.0 "Discount")))))

(fn PerformAgentAction
  (params (InActionObject :type Learning%20Agents%20Action%20Object%20Object%20Reference) (InActionObjectElement :type Learning%20Agents%20Action%20Object%20Element%20Structure%20%28by%20ref%29) (AgentId :type Integer))
  (LocalVariables|SetActActor (Class|LearningAgentsManagerListener|GetAgent AgentId "/Game/Blueprints/FSMBPs/BP_FSMPawn.BP_FSMPawn_C"))
  (if (Utilities|Enum|Equal(Enum) (Variables|/Game/Blueprints/FSMBPs/BP_FSMPawn.BP_FSMPawn_C|GetFSMState (LocalVariables|GetActActor)) (Variables|/Game/Blueprints/FSMBPs/BP_FSMPawn.BP_FSMPawn_C|GetPreviousState (LocalVariables|GetActActor)))
    _
    (else
      (Variables|/Game/Blueprints/FSMBPs/BP_FSMPawn.BP_FSMPawn_C|SetPreviousState (LocalVariables|GetActActor) (Variables|/Game/Blueprints/FSMBPs/BP_FSMPawn.BP_FSMPawn_C|GetFSMState (LocalVariables|GetActActor)))))
  (bind _outelements (Class|LearningAgentsActions|GetStructAction InActionObject InActionObjectElement))
  (bind _outenumvalue (Class|LearningAgentsActions|GetEnumAction InActionObject (.Value (Utilities|Map|Find _outelements "ChangeState")) "/Game/Blueprints/FSMBPs/FSMState.FSMState" "EnumAction" false 0))
  (bind _output_get (Variables|/Game/Blueprints/FSMBPs/BP_FSMPawn.BP_FSMPawn_C|SetFSMState (LocalVariables|GetActActor) (Utilities|Enum|ByteToEnumFSMState _outenumvalue)))
  (switch Utilities|FlowControl|Switch|SwitchonFSMState _output_get
    (:NewEnumerator2
      ;[0.15 0.15 0.15 0.5] ResetShop
      (if (Utilities|Array|IsNotEmpty (Variables|/Game/Blueprints/FSMBPs/BP_FSMPawn.BP_FSMPawn_C|GetShopItemNames (LocalVariables|GetActActor)))
        (Utilities|Array|Clear (Variables|/Game/Blueprints/FSMBPs/BP_FSMPawn.BP_FSMPawn_C|GetShopItemNames (LocalVariables|GetActActor)))
        (Utilities|Array|Clear (Variables|/Game/Blueprints/FSMBPs/BP_FSMPawn.BP_FSMPawn_C|GetShopItemPrices (LocalVariables|GetActActor))))
      (Variables|/Game/Blueprints/FSMBPs/BP_FSMPawn.BP_FSMPawn_C|SetShopText (LocalVariables|GetActActor) "")
      (Variables|/Game/Blueprints/FSMBPs/BP_FSMPawn.BP_FSMPawn_C|SetAppliedDiscount? (LocalVariables|GetActActor) false)
      (Variables|/Game/Blueprints/FSMBPs/BP_FSMPawn.BP_FSMPawn_C|SetResetShop? (LocalVariables|GetActActor) true))
    (:NewEnumerator7
      ;[0.15 0.15 0.15 0.5] Get Player Stats
      (Variables|/Game/Blueprints/FSMBPs/BP_FSMPawn.BP_FSMPawn_C|SetPlayerWeaponClass (LocalVariables|GetActActor) (Variables|/Script/MScDiss.FSMPlayerPawnComponent|GetWeaponClass (Variables|Default|GetPlayer)))
      (Variables|/Game/Blueprints/FSMBPs/BP_FSMPawn.BP_FSMPawn_C|SetPlayerCurrentGold (LocalVariables|GetActActor) (Variables|/Script/MScDiss.FSMPlayerPawnComponent|GetCurrentGold (Variables|Default|GetPlayer)))
      (Variables|/Game/Blueprints/FSMBPs/BP_FSMPawn.BP_FSMPawn_C|SetPlayerReputation (LocalVariables|GetActActor) (Variables|/Script/MScDiss.FSMPlayerPawnComponent|GetReputation (Variables|Default|GetPlayer)))
      (Variables|/Game/Blueprints/FSMBPs/BP_FSMPawn.BP_FSMPawn_C|SetObservedPlayer? (LocalVariables|GetActActor) true))
    (:NewEnumerator4
      ;[0.15 0.15 0.15 0.5] Deciding Items and Prices
      (bind _outelements_2 (Class|LearningAgentsActions|GetStructAction InActionObject InActionObjectElement))
      (bind _outvalue (Class|LearningAgentsActions|GetFloatAction InActionObject (.Value (Utilities|Map|Find _outelements_2 "ItemName0")) "ItemName0" false 0))
      (if (> (Math|Float|Clamp(Float) _outvalue) 0.5)
        (Variables|/Game/Blueprints/FSMBPs/BP_FSMPawn.BP_FSMPawn_C|SetSelectedWeaponIndex (LocalVariables|GetActActor) 1)
        (Utilities|Array|Add (Variables|/Game/Blueprints/FSMBPs/BP_FSMPawn.BP_FSMPawn_C|GetShopItemNames (LocalVariables|GetActActor)) (Utilities|Array|Get(acopy) (Variables|/Game/Blueprints/FSMBPs/BP_FSMPawn.BP_FSMPawn_C|GetWeaponNames (LocalVariables|GetActActor)) 1))
        (else
          (Variables|/Game/Blueprints/FSMBPs/BP_FSMPawn.BP_FSMPawn_C|SetSelectedWeaponIndex (LocalVariables|GetActActor) 0)
          (Utilities|Array|Add (Variables|/Game/Blueprints/FSMBPs/BP_FSMPawn.BP_FSMPawn_C|GetShopItemNames (LocalVariables|GetActActor)) (Utilities|Array|Get(acopy) (Variables|/Game/Blueprints/FSMBPs/BP_FSMPawn.BP_FSMPawn_C|GetWeaponNames (LocalVariables|GetActActor))))))
      (bind _outvalue_2 (Class|LearningAgentsActions|GetFloatAction InActionObject (.Value (Utilities|Map|Find _outelements_2 "ItemName1")) "ItemName1" false 0))
      (Utilities|Array|Add (Variables|/Game/Blueprints/FSMBPs/BP_FSMPawn.BP_FSMPawn_C|GetShopItemNames (LocalVariables|GetActActor)) (Utilities|Array|Get(acopy) (Variables|/Game/Blueprints/FSMBPs/BP_FSMPawn.BP_FSMPawn_C|GetItemNames (LocalVariables|GetActActor)) (Math|Float|Round (* (Math|Float|Clamp(Float) (Math|Float|Absolute(Float) _outvalue_2) 0.0 3.0) 2.5))))
      (bind _outvalue_3 (Class|LearningAgentsActions|GetFloatAction InActionObject (.Value (Utilities|Map|Find _outelements_2 "ItemName2")) "ItemName2" false 0))
      (Utilities|Array|Add (Variables|/Game/Blueprints/FSMBPs/BP_FSMPawn.BP_FSMPawn_C|GetShopItemNames (LocalVariables|GetActActor)) (Utilities|Array|Get(acopy) (Variables|/Game/Blueprints/FSMBPs/BP_FSMPawn.BP_FSMPawn_C|GetItemNames (LocalVariables|GetActActor)) (Math|Float|Round (* (Math|Float|Clamp(Float) (Math|Float|Absolute(Float) _outvalue_3) 0.0 3.0) 2.5))))
      (bind _outvalue_4 (Class|LearningAgentsActions|GetFloatAction InActionObject (.Value (Utilities|Map|Find _outelements_2 "ItemPrice0")) "ItemPrice0" false 0))
      (Utilities|Array|Add (Variables|/Game/Blueprints/FSMBPs/BP_FSMPawn.BP_FSMPawn_C|GetShopItemPrices (LocalVariables|GetActActor)) (Math|Float|Round (* (Math|Float|Clamp(Float) (Math|Float|Absolute(Float) _outvalue_4)) (Math|Random|RandomFloatinRange 9e+02 1e+03))))
      (bind _outvalue_5 (Class|LearningAgentsActions|GetFloatAction InActionObject (.Value (Utilities|Map|Find _outelements_2 "ItemPrice1")) "ItemPrice1" false 0))
      (Utilities|Array|Add (Variables|/Game/Blueprints/FSMBPs/BP_FSMPawn.BP_FSMPawn_C|GetShopItemPrices (LocalVariables|GetActActor)) (Math|Float|Round (* (Math|Float|Clamp(Float) (Math|Float|Absolute(Float) _outvalue_5)) (Math|Random|RandomFloatinRange 9e+02 1e+03))))
      (bind _outvalue_6 (Class|LearningAgentsActions|GetFloatAction InActionObject (.Value (Utilities|Map|Find _outelements_2 "ItemPrice2")) "ItemPrice2" false 0))
      (Utilities|Array|Add (Variables|/Game/Blueprints/FSMBPs/BP_FSMPawn.BP_FSMPawn_C|GetShopItemPrices (LocalVariables|GetActActor)) (Math|Float|Round (* (Math|Float|Clamp(Float) (Math|Float|Absolute(Float) _outvalue_6)) (Math|Random|RandomFloatinRange 9e+02 1e+03))))
      (Variables|/Game/Blueprints/FSMBPs/BP_FSMPawn.BP_FSMPawn_C|SetDecideItems? (LocalVariables|GetActActor) true))
    (:NewEnumerator5
      ;[0.15 0.15 0.15 0.5] Decide Discount
      (if (not (Variables|/Game/Blueprints/FSMBPs/BP_FSMPawn.BP_FSMPawn_C|GetAppliedDiscount? (LocalVariables|GetActActor)))
        (for _index (range 0 3)
          (if (== (Math|Random|RandomIntegerinRange 0 5) 1)
            (bind _outelements_3 (Class|LearningAgentsActions|GetStructAction InActionObject InActionObjectElement))
            (bind _outvalue_7 (Class|LearningAgentsActions|GetFloatAction InActionObject (.Value (Utilities|Map|Find _outelements_3 "Discount")) "Discount" false 0))
            (Variables|/Game/Blueprints/FSMBPs/BP_FSMPawn.BP_FSMPawn_C|SetDiscountMult (LocalVariables|GetActActor) (Math|Float|Clamp(Float) _outvalue_7 0.0 2.0))
            (Utilities|Array|SetArrayElem (Variables|/Game/Blueprints/FSMBPs/BP_FSMPawn.BP_FSMPawn_C|GetShopItemPrices (LocalVariables|GetActActor)) _index (Math|Float|Truncate (* (Utilities|Array|Get(acopy) (Variables|/Game/Blueprints/FSMBPs/BP_FSMPawn.BP_FSMPawn_C|GetShopItemPrices (LocalVariables|GetActActor)) _index) (Math|Float|Clamp(Float) _outvalue_7 0.0 2.0))))
            (Variables|/Game/Blueprints/FSMBPs/BP_FSMPawn.BP_FSMPawn_C|SetShopText (LocalVariables|GetActActor) "Discount Applied!")))
        (Variables|/Game/Blueprints/FSMBPs/BP_FSMPawn.BP_FSMPawn_C|SetAppliedDiscount? (LocalVariables|GetActActor) true)
        (Variables|/Game/Blueprints/FSMBPs/BP_FSMPawn.BP_FSMPawn_C|SetDecideDiscount? (LocalVariables|GetActActor) true)))
    (:NewEnumerator6
      (Variables|/Game/Blueprints/FSMBPs/BP_FSMPawn.BP_FSMPawn_C|SetProcessComplete? (LocalVariables|GetActActor) true))))