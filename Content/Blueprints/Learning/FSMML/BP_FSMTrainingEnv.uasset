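; Learning Agents training environment that trains BP_FSMPawn agents to run a shop decision state machine.
; Rewards score whether weapon selection and shop item fit the player's class, plus FSM states whose step flag is set, and are printed for debugging; discount reward terms sit unconnected.
; Episodes truncate when all steps complete and terminate when a state lacks its flag.
; Reset clears the completion flag and calls the agent's player respawn.
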(fn GatherAgentReward
  (params (AgentId :type Integer))
  (LocalVariables|SetRewardActor (Class|LearningAgentsManagerListener|GetAgent AgentId "/Game/Blueprints/FSMBPs/BP_FSMPawn.BP_FSMPawn_C"))
  (Development|PrintString 0 (Utilities|String|ToString(Float) (+ (+ (Class|LearningAgentsRewards|MakeRewardonCondition (Math|Boolean|ANDBoolean (== (Variables|/Game/Blueprints/FSMBPs/BP_FSMPawn.BP_FSMPawn_C|GetSelectedWeaponIndex (LocalVariables|GetRewardActor)) 0) (== (Variables|/Game/Blueprints/FSMBPs/BP_FSMPawn.BP_FSMPawn_C|GetPlayerWeaponClass (LocalVariables|GetRewardActor)) 0) (Utilities|Enum|Equal(Enum) (Utilities|Array|Get(acopy) (Variables|/Game/Blueprints/FSMBPs/BP_FSMPawn.BP_FSMPawn_C|GetShopItemNames (LocalVariables|GetRewardActor))) (Utilities|Array|Get(acopy) (Variables|/Game/Blueprints/FSMBPs/BP_FSMPawn.BP_FSMPawn_C|GetWeaponNames (LocalVariables|GetRewardActor)) (Variables|/Game/Blueprints/FSMBPs/BP_FSMPawn.BP_FSMPawn_C|GetPlayerWeaponClass (LocalVariables|GetRewardActor))))) 2.0 "ConditionReward" false 0) (Class|LearningAgentsRewards|MakeRewardonCondition (Math|Boolean|ANDBoolean (== (Variables|/Game/Blueprints/FSMBPs/BP_FSMPawn.BP_FSMPawn_C|GetSelectedWeaponIndex (LocalVariables|GetRewardActor)) 1) (== (Variables|/Game/Blueprints/FSMBPs/BP_FSMPawn.BP_FSMPawn_C|GetPlayerWeaponClass (LocalVariables|GetRewardActor)) 1) (Utilities|Enum|Equal(Enum) (Utilities|Array|Get(acopy) (Variables|/Game/Blueprints/FSMBPs/BP_FSMPawn.BP_FSMPawn_C|GetShopItemNames (LocalVariables|GetRewardActor)) 1) (Utilities|Array|Get(acopy) (Variables|/Game/Blueprints/FSMBPs/BP_FSMPawn.BP_FSMPawn_C|GetWeaponNames (LocalVariables|GetRewardActor)) (Variables|/Game/Blueprints/FSMBPs/BP_FSMPawn.BP_FSMPawn_C|GetPlayerWeaponClass (LocalVariables|GetRewardActor))))) 2.0 "ConditionReward" false 0) (Class|LearningAgentsRewards|MakeRewardonCondition (Class|KismetMathLibrary|XORBoolean (Class|KismetMathLibrary|XORBoolean (== (Variables|/Game/Blueprints/FSMBPs/BP_FSMPawn.BP_FSMPawn_C|GetSelectedWeaponIndex (LocalVariables|GetRewardActor)) 0) (== (Variables|/Game/Blueprints/FSMBPs/BP_FSMPawn.BP_FSMPawn_C|GetPlayerWeaponClass (LocalVariables|GetRewardActor)) 0)) (Utilities|Enum|Equal(Enum) (Utilities|Array|Get(acopy) (Variables|/Game/Blueprints/FSMBPs/BP_FSMPawn.BP_FSMPawn_C|GetShopItemNames (LocalVariables|GetRewardActor))) (Utilities|Array|Get(acopy) (Variables|/Game/Blueprints/FSMBPs/BP_FSMPawn.BP_FSMPawn_C|GetWeaponNames (LocalVariables|GetRewardActor)) (Variables|/Game/Blueprints/FSMBPs/BP_FSMPawn.BP_FSMPawn_C|GetPlayerWeaponClass (LocalVariables|GetRewardActor))))) -4.0 "ConditionReward" false 0) (Class|LearningAgentsRewards|MakeRewardonCondition (Class|KismetMathLibrary|XORBoolean (Class|KismetMathLibrary|XORBoolean (== (Variables|/Game/Blueprints/FSMBPs/BP_FSMPawn.BP_FSMPawn_C|GetSelectedWeaponIndex (LocalVariables|GetRewardActor)) 1) (== (Variables|/Game/Blueprints/FSMBPs/BP_FSMPawn.BP_FSMPawn_C|GetPlayerWeaponClass (LocalVariables|GetRewardActor)) 1)) (Utilities|Enum|Equal(Enum) (Utilities|Array|Get(acopy) (Variables|/Game/Blueprints/FSMBPs/BP_FSMPawn.BP_FSMPawn_C|GetShopItemNames (LocalVariables|GetRewardActor)) 1) (Utilities|Array|Get(acopy) (Variables|/Game/Blueprints/FSMBPs/BP_FSMPawn.BP_FSMPawn_C|GetWeaponNames (LocalVariables|GetRewardActor)) (Variables|/Game/Blueprints/FSMBPs/BP_FSMPawn.BP_FSMPawn_C|GetPlayerWeaponClass (LocalVariables|GetRewardActor))))) -4.0 "ConditionReward" false 0)) 0.0 0.0 (Class|LearningAgentsRewards|MakeRewardonCondition (Math|Boolean|ORBoolean (and (Utilities|Enum|Equal(Enum) (Variables|/Game/Blueprints/FSMBPs/BP_FSMPawn.BP_FSMPawn_C|GetFSMState (LocalVariables|GetRewardActor)) "NewEnumerator7") (Variables|/Game/Blueprints/FSMBPs/BP_FSMPawn.BP_FSMPawn_C|GetResetShop? (LocalVariables|GetRewardActor))) (and (Utilities|Enum|Equal(Enum) (Variables|/Game/Blueprints/FSMBPs/BP_FSMPawn.BP_FSMPawn_C|GetFSMState (LocalVariables|GetRewardActor)) "NewEnumerator4") (Variables|/Game/Blueprints/FSMBPs/BP_FSMPawn.BP_FSMPawn_C|GetObservedPlayer? (LocalVariables|GetRewardActor))) (and (Utilities|Enum|Equal(Enum) (Variables|/Game/Blueprints/FSMBPs/BP_FSMPawn.BP_FSMPawn_C|GetFSMState (LocalVariables|GetRewardActor)) "NewEnumerator5") (Variables|/Game/Blueprints/FSMBPs/BP_FSMPawn.BP_FSMPawn_C|GetDecideItems? (LocalVariables|GetRewardActor))) (and (Utilities|Enum|Equal(Enum) (Variables|/Game/Blueprints/FSMBPs/BP_FSMPawn.BP_FSMPawn_C|GetFSMState (LocalVariables|GetRewardActor)) "NewEnumerator6") (Variables|/Game/Blueprints/FSMBPs/BP_FSMPawn.BP_FSMPawn_C|GetDecideDiscount? (LocalVariables|GetRewardActor)))) 5.0 "ConditionReward" false 0) 0.0 0.0)))
  (return (+ (+ (Class|LearningAgentsRewards|MakeRewardonCondition (Math|Boolean|ANDBoolean (== (Variables|/Game/Blueprints/FSMBPs/BP_FSMPawn.BP_FSMPawn_C|GetSelectedWeaponIndex (LocalVariables|GetRewardActor)) 0) (== (Variables|/Game/Blueprints/FSMBPs/BP_FSMPawn.BP_FSMPawn_C|GetPlayerWeaponClass (LocalVariables|GetRewardActor)) 0) (Utilities|Enum|Equal(Enum) (Utilities|Array|Get(acopy) (Variables|/Game/Blueprints/FSMBPs/BP_FSMPawn.BP_FSMPawn_C|GetShopItemNames (LocalVariables|GetRewardActor))) (Utilities|Array|Get(acopy) (Variables|/Game/Blueprints/FSMBPs/BP_FSMPawn.BP_FSMPawn_C|GetWeaponNames (LocalVariables|GetRewardActor)) (Variables|/Game/Blueprints/FSMBPs/BP_FSMPawn.BP_FSMPawn_C|GetPlayerWeaponClass (LocalVariables|GetRewardActor))))) 2.0 "ConditionReward" false 0) (Class|LearningAgentsRewards|MakeRewardonCondition (Math|Boolean|ANDBoolean (== (Variables|/Game/Blueprints/FSMBPs/BP_FSMPawn.BP_FSMPawn_C|GetSelectedWeaponIndex (LocalVariables|GetRewardActor)) 1) (== (Variables|/Game/Blueprints/FSMBPs/BP_FSMPawn.BP_FSMPawn_C|GetPlayerWeaponClass (LocalVariables|GetRewardActor)) 1) (Utilities|Enum|Equal(Enum) (Utilities|Array|Get(acopy) (Variables|/Game/Blueprints/FSMBPs/BP_FSMPawn.BP_FSMPawn_C|GetShopItemNames (LocalVariables|GetRewardActor)) 1) (Utilities|Array|Get(acopy) (Variables|/Game/Blueprints/FSMBPs/BP_FSMPawn.BP_FSMPawn_C|GetWeaponNames (LocalVariables|GetRewardActor)) (Variables|/Game/Blueprints/FSMBPs/BP_FSMPawn.BP_FSMPawn_C|GetPlayerWeaponClass (LocalVariables|GetRewardActor))))) 2.0 "ConditionReward" false 0) (Class|LearningAgentsRewards|MakeRewardonCondition (Class|KismetMathLibrary|XORBoolean (Class|KismetMathLibrary|XORBoolean (== (Variables|/Game/Blueprints/FSMBPs/BP_FSMPawn.BP_FSMPawn_C|GetSelectedWeaponIndex (LocalVariables|GetRewardActor)) 0) (== (Variables|/Game/Blueprints/FSMBPs/BP_FSMPawn.BP_FSMPawn_C|GetPlayerWeaponClass (LocalVariables|GetRewardActor)) 0)) (Utilities|Enum|Equal(Enum) (Utilities|Array|Get(acopy) (Variables|/Game/Blueprints/FSMBPs/BP_FSMPawn.BP_FSMPawn_C|GetShopItemNames (LocalVariables|GetRewardActor))) (Utilities|Array|Get(acopy) (Variables|/Game/Blueprints/FSMBPs/BP_FSMPawn.BP_FSMPawn_C|GetWeaponNames (LocalVariables|GetRewardActor)) (Variables|/Game/Blueprints/FSMBPs/BP_FSMPawn.BP_FSMPawn_C|GetPlayerWeaponClass (LocalVariables|GetRewardActor))))) -4.0 "ConditionReward" false 0) (Class|LearningAgentsRewards|MakeRewardonCondition (Class|KismetMathLibrary|XORBoolean (Class|KismetMathLibrary|XORBoolean (== (Variables|/Game/Blueprints/FSMBPs/BP_FSMPawn.BP_FSMPawn_C|GetSelectedWeaponIndex (LocalVariables|GetRewardActor)) 1) (== (Variables|/Game/Blueprints/FSMBPs/BP_FSMPawn.BP_FSMPawn_C|GetPlayerWeaponClass (LocalVariables|GetRewardActor)) 1)) (Utilities|Enum|Equal(Enum) (Utilities|Array|Get(acopy) (Variables|/Game/Blueprints/FSMBPs/BP_FSMPawn.BP_FSMPawn_C|GetShopItemNames (LocalVariables|GetRewardActor)) 1) (Utilities|Array|Get(acopy) (Variables|/Game/Blueprints/FSMBPs/BP_FSMPawn.BP_FSMPawn_C|GetWeaponNames (LocalVariables|GetRewardActor)) (Variables|/Game/Blueprints/FSMBPs/BP_FSMPawn.BP_FSMPawn_C|GetPlayerWeaponClass (LocalVariables|GetRewardActor))))) -4.0 "ConditionReward" false 0)) 0.0 0.0 (Class|LearningAgentsRewards|MakeRewardonCondition (Math|Boolean|ORBoolean (and (Utilities|Enum|Equal(Enum) (Variables|/Game/Blueprints/FSMBPs/BP_FSMPawn.BP_FSMPawn_C|GetFSMState (LocalVariables|GetRewardActor)) "NewEnumerator7") (Variables|/Game/Blueprints/FSMBPs/BP_FSMPawn.BP_FSMPawn_C|GetResetShop? (LocalVariables|GetRewardActor))) (and (Utilities|Enum|Equal(Enum) (Variables|/Game/Blueprints/FSMBPs/BP_FSMPawn.BP_FSMPawn_C|GetFSMState (LocalVariables|GetRewardActor)) "NewEnumerator4") (Variables|/Game/Blueprints/FSMBPs/BP_FSMPawn.BP_FSMPawn_C|GetObservedPlayer? (LocalVariables|GetRewardActor))) (and (Utilities|Enum|Equal(Enum) (Variables|/Game/Blueprints/FSMBPs/BP_FSMPawn.BP_FSMPawn_C|GetFSMState (LocalVariables|GetRewardActor)) "NewEnumerator5") (Variables|/Game/Blueprints/FSMBPs/BP_FSMPawn.BP_FSMPawn_C|GetDecideItems? (LocalVariables|GetRewardActor))) (and (Utilities|Enum|Equal(Enum) (Variables|/Game/Blueprints/FSMBPs/BP_FSMPawn.BP_FSMPawn_C|GetFSMState (LocalVariables|GetRewardActor)) "NewEnumerator6") (Variables|/Game/Blueprints/FSMBPs/BP_FSMPawn.BP_FSMPawn_C|GetDecideDiscount? (LocalVariables|GetRewardActor)))) 5.0 "ConditionReward" false 0) 0.0 0.0)))

(fn GatherAgentCompletion
  (params (AgentId :type Integer))
  (bind _output_get (LocalVariables|SetCompActor (Class|LearningAgentsManagerListener|GetAgent AgentId "/Game/Blueprints/FSMBPs/BP_FSMPawn.BP_FSMPawn_C")))
  (return (Class|LearningAgentsCompletions|Completionor (Class|LearningAgentsCompletions|MakeCompletiononCondition (Math|Boolean|ANDBoolean (Variables|/Game/Blueprints/FSMBPs/BP_FSMPawn.BP_FSMPawn_C|GetProcessComplete? _output_get) (Variables|/Game/Blueprints/FSMBPs/BP_FSMPawn.BP_FSMPawn_C|GetResetShop? _output_get) (Variables|/Game/Blueprints/FSMBPs/BP_FSMPawn.BP_FSMPawn_C|GetObservedPlayer? _output_get) (Variables|/Game/Blueprints/FSMBPs/BP_FSMPawn.BP_FSMPawn_C|GetDecideItems? _output_get) (Variables|/Game/Blueprints/FSMBPs/BP_FSMPawn.BP_FSMPawn_C|GetDecideDiscount? _output_get)) "Truncation" "ConditionCompletion" false 0) (Class|LearningAgentsCompletions|MakeCompletiononCondition (Math|Boolean|ORBoolean (and (Utilities|Enum|Equal(Enum) (Variables|/Game/Blueprints/FSMBPs/BP_FSMPawn.BP_FSMPawn_C|GetFSMState (LocalVariables|GetCompActor)) "NewEnumerator7") (not (Variables|/Game/Blueprints/FSMBPs/BP_FSMPawn.BP_FSMPawn_C|GetResetShop? (LocalVariables|GetCompActor)))) (and (Utilities|Enum|Equal(Enum) (Variables|/Game/Blueprints/FSMBPs/BP_FSMPawn.BP_FSMPawn_C|GetFSMState (LocalVariables|GetCompActor)) "NewEnumerator4") (not (Variables|/Game/Blueprints/FSMBPs/BP_FSMPawn.BP_FSMPawn_C|GetObservedPlayer? (LocalVariables|GetCompActor)))) (and (Utilities|Enum|Equal(Enum) (Variables|/Game/Blueprints/FSMBPs/BP_FSMPawn.BP_FSMPawn_C|GetFSMState (LocalVariables|GetCompActor)) "NewEnumerator5") (not (Variables|/Game/Blueprints/FSMBPs/BP_FSMPawn.BP_FSMPawn_C|GetDecideItems? (LocalVariables|GetCompActor)))) (and (Utilities|Enum|Equal(Enum) (Variables|/Game/Blueprints/FSMBPs/BP_FSMPawn.BP_FSMPawn_C|GetFSMState (LocalVariables|GetCompActor)) "NewEnumerator6") (not (Variables|/Game/Blueprints/FSMBPs/BP_FSMPawn.BP_FSMPawn_C|GetDecideDiscount? (LocalVariables|GetCompActor))))) "Termination" "ConditionCompletion" false 0))))

(fn ResetAgentEpisode
  (params (AgentId :type Integer))
  (bind _returnvalue (Class|LearningAgentsManagerListener|GetAgent AgentId "/Game/Blueprints/FSMBPs/BP_FSMPawn.BP_FSMPawn_C"))
  (Variables|/Game/Blueprints/FSMBPs/BP_FSMPawn.BP_FSMPawn_C|SetProcessComplete? _returnvalue false)
  (Default|RespawnPlayerPawn _returnvalue))