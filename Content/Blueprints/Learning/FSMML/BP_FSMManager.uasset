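; BP_FSMManager is a Learning Agents manager that trains or runs a neural policy for FSM pawns in a level with a player pawn.
; BeginPlay makes itself their tick prerequisite, shows the BP_MLShop widget and builds the interactor, policy, critic, training environment and shared-memory PPO trainer.
; RunInference switches Tick from training to inference, keeps saved networks instead of reinitializing them, and triggers player respawn at startup.
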(event EventTick
  (params (DeltaSeconds :type Float%20%28single-precision%29))
  (if (Variables|Default|GetRun%20Inference)
    (Class|LearningAgentsPolicy|RunInference (Variables|Default|GetPolicy) 0.0)
    (else
      (Class|LearningAgentsPPOTrainer|RunTraining (Variables|Default|GetPPOTrainer) (Variables|Default|GetTrainer%20Training%20Settings) (Variables|Default|GetTraining%20Game%20Settings) true true))))

(event EventBeginPlay
  (bind _shared_memory_settings (Variables|Default|GetShared%20Memory%20Settings))
  (bind _run_inference (Variables|Default|GetRun%20Inference))
  (bind _returnvalue (not _run_inference))
  (Utilities|FlowControl|Sequence
    (:then_0
      (bind _outactors (Actor|GetAllActorsOfClass "/Game/Blueprints/FSMBPs/BP_FSMPawn.BP_FSMPawn_C"))
      (bind _output_get (Variables|Default|SetFSMActors _outactors))
      (Actor|Tick|AddTickPrerequisiteActor _output_get self))
    (:then_1
      (bind _returnvalue_2 (UserInterface|CreateWidget "/Game/Blueprints/FSMBPs/BP_MLShop.BP_MLShop_C" 0 0))
      (UserInterface|Viewport|AddtoViewport _returnvalue_2 0))
    (:then_2
      (bind _returnvalue_3 (Actor|GetActorOfClass "/Game/Blueprints/FSMBPs/BP_FSMPlayerPawn.BP_FSMPlayerPawn_C"))
      (Variables|Default|SetPlayer _returnvalue_3))
    (:then_3
      (bind _returnvalue_4 (Class|LearningAgentsInteractor|MakeInteractor (Variables|Default|GetLearningAgentsManager) "/Game/Blueprints/Learning/FSMML/BP_FSMInteractor.BP_FSMInteractor_C" "AStarInteractor"))
      (bind _output_get_2 (Variables|Default|SetInteractor _returnvalue_4))
      (Variables|/Game/Blueprints/Learning/FSMML/BP_FSMInteractor.BP_FSMInteractor_C|SetPlayer _output_get_2 (Actor|GetComponentbyClass (Variables|Default|GetPlayer) "/Script/MScDiss.FSMPlayerPawnComponent")))
    (:then_4
      (bind _returnvalue_5 (Class|LearningAgentsPolicy|MakePolicy (Variables|Default|GetLearningAgentsManager) (Variables|Default|GetInteractor) "/Script/LearningAgents.LearningAgentsPolicy" "FSMPolicy" "/Game/Blueprints/Learning/FSMML/DA_FSMEncoder.DA_FSMEncoder" "/Game/Blueprints/Learning/FSMML/DA_FSMPolicy.DA_FSMPolicy" "/Game/Blueprints/Learning/FSMML/DA_FSMDecoder.DA_FSMDecoder" _returnvalue _returnvalue _returnvalue (Variables|Default|GetPolicy%20Settings) 1234))
      (Variables|Default|SetPolicy _returnvalue_5))
    (:then_5
      (bind _returnvalue_6 (Class|LearningAgentsCritic|MakeCritic (Variables|Default|GetLearningAgentsManager) (Variables|Default|GetInteractor) (Variables|Default|GetPolicy) "/Script/LearningAgents.LearningAgentsCritic" "FSMCritic" "/Game/Blueprints/Learning/FSMML/DA_FSMCritic.DA_FSMCritic" (not (Variables|Default|GetRun%20Inference)) (Variables|Default|GetCritic%20Settings) 1234))
      (Variables|Default|SetCritic _returnvalue_6))
    (:then_6
      (bind _returnvalue_7 (Class|LearningAgentsTrainingEnvironment|MakeTrainingEnvironment (Variables|Default|GetLearningAgentsManager) "/Game/Blueprints/Learning/FSMML/BP_FSMTrainingEnv.BP_FSMTrainingEnv_C" "TrainingEnvironment"))
      (Variables|Default|SetTrainingEnv _returnvalue_7))
    (:then_7
      (bind _returnvalue_8 (Class|LearningAgentsCommunicatorLibrary|SpawnSharedMemoryTrainingProcess (Variables|Default|GetTrainer%20Process%20Settings) _shared_memory_settings))
      (bind _returnvalue_9 (Class|LearningAgentsCommunicatorLibrary|MakeSharedMemoryCommunicator _returnvalue_8 _shared_memory_settings))
      (Variables|Default|SetCommunicator _returnvalue_9))
    (:then_8
      (bind _returnvalue_10 (Class|LearningAgentsPPOTrainer|MakePPOTrainer (Variables|Default|GetLearningAgentsManager) (Variables|Default|GetInteractor) (Variables|Default|GetTrainingEnv) (Variables|Default|GetPolicy) (Variables|Default|GetCritic) (Variables|Default|GetCommunicator) "/Script/LearningAgentsTraining.LearningAgentsPPOTrainer" "PPOTrainer" (Variables|Default|GetTrainer%20Settings)))
      (Variables|Default|SetPPOTrainer _returnvalue_10))
    (:then_9
      (if (Variables|Default|GetRun%20Inference)
        (Default|RespawnPlayerPawn (Variables|Default|GetFSMActors))))))

(fn ConstructionScript)