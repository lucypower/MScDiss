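; BP_AStarManager is the Learning Agents manager actor that trains or runs a neural-network policy for AStar pawns on a generated grid.
; BeginPlay finds the pawns and map, makes the pawns tick after it, then builds the interactor, policy, critic, training environment and shared-memory PPO trainer.
; RunInference keeps saved networks and runs the policy each tick.
; Otherwise networks reinitialize and PPO trains, with a looping timer periodically resetting grid and pawn starts.
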(event Custom|CustomEvent
  (Class|AStarMapGeneration|ResetGrid (Variables|Default|GetGridRef))
  (Default|ResettoNewStartLocation (Variables|Default|GetAStarActors)))

(event EventBeginPlay
  (bind _shared_memory_settings (Variables|Default|GetShared%20Memory%20Settings))
  (bind _runinference (Variables|Default|GetRunInference))
  (bind _returnvalue (not _runinference))
  (Utilities|FlowControl|Sequence
    (:then_0
      (bind _outactors (Actor|GetAllActorsOfClass "/Game/Blueprints/AStarBPs/BP_AStarPawn.BP_AStarPawn_C"))
      (bind _output_get (Variables|Default|SetAStarActors _outactors))
      (Actor|Tick|AddTickPrerequisiteActor _output_get self))
    (:then_1
      (bind _returnvalue_2 (Actor|GetActorOfClass "/Game/Blueprints/AStarBPs/BP_AStarMapGen.BP_AStarMapGen_C"))
      (Variables|Default|SetGridRef _returnvalue_2))
    (:then_2
      (bind _returnvalue_3 (Class|LearningAgentsInteractor|MakeInteractor (Variables|Default|GetLearningAgentsManager) "/Game/Blueprints/Learning/AStarML/BP_AStarInteractor.BP_AStarInteractor_C" "AStarInteractor"))
      (Variables|Default|SetInteractor _returnvalue_3))
    (:then_3
      (bind _returnvalue_4 (Class|LearningAgentsPolicy|MakePolicy (Variables|Default|GetLearningAgentsManager) (Variables|Default|GetInteractor) "/Script/LearningAgents.LearningAgentsPolicy" "AStarPolicy" "/Game/Blueprints/Learning/AStarML/DA_AStarEncoder.DA_AStarEncoder" "/Game/Blueprints/Learning/AStarML/DA_AStarPolicy.DA_AStarPolicy" "/Game/Blueprints/Learning/AStarML/DA_AStarDecoder.DA_AStarDecoder" _returnvalue _returnvalue _returnvalue (Variables|Default|GetPolicy%20Settings) 1234))
      (Variables|Default|SetPolicy _returnvalue_4))
    (:then_4
      (bind _returnvalue_5 (Class|LearningAgentsCritic|MakeCritic (Variables|Default|GetLearningAgentsManager) (Variables|Default|GetInteractor) (Variables|Default|GetPolicy) "/Script/LearningAgents.LearningAgentsCritic" "AStarCritic" "/Game/Blueprints/Learning/AStarML/DA_AStarCritic.DA_AStarCritic" (not (Variables|Default|GetRunInference)) (Variables|Default|GetCritic%20Settings) 1234))
      (Variables|Default|SetCritic _returnvalue_5))
    (:then_5
      (bind _returnvalue_6 (Class|LearningAgentsTrainingEnvironment|MakeTrainingEnvironment (Variables|Default|GetLearningAgentsManager) "/Game/Blueprints/Learning/AStarML/BP_AStarTrainingEnv.BP_AStarTrainingEnv_C" "TrainingEnvironment"))
      (Variables|Default|SetTrainingEnv _returnvalue_6))
    (:then_6
      (bind _returnvalue_7 (Class|LearningAgentsCommunicatorLibrary|SpawnSharedMemoryTrainingProcess (Variables|Default|GetTrainer%20Process%20Settings) _shared_memory_settings))
      (bind _returnvalue_8 (Class|LearningAgentsCommunicatorLibrary|MakeSharedMemoryCommunicator _returnvalue_7 _shared_memory_settings))
      (Variables|Default|SetCommunicator _returnvalue_8))
    (:then_7
      (bind _returnvalue_9 (Class|LearningAgentsPPOTrainer|MakePPOTrainer (Variables|Default|GetLearningAgentsManager) (Variables|Default|GetInteractor) (Variables|Default|GetTrainingEnv) (Variables|Default|GetPolicy) (Variables|Default|GetCritic) (Variables|Default|GetCommunicator) "/Script/LearningAgentsTraining.LearningAgentsPPOTrainer" "PPOTrainer" (Variables|Default|GetTrainer%20Settings)))
      (Variables|Default|SetPPOTrainer _returnvalue_9))
    (:then_8
      (if (Variables|Default|GetRunInference)
        (Default|ResettoNewStartLocation (Variables|Default|GetAStarActors))))))

(event EventTick
  (params (DeltaSeconds :type Float%20%28single-precision%29))
  (if (Variables|Default|GetRunInference)
    (Class|LearningAgentsPolicy|RunInference (Variables|Default|GetPolicy) 0.0)
    (else
      (Class|LearningAgentsPPOTrainer|RunTraining (Variables|Default|GetPPOTrainer) (Variables|Default|GetTrainer%20Training%20Settings) (Variables|Default|GetTraining%20Game%20Settings) true true)
      (Utilities|FlowControl|DoOnce false
        (:Completed
          (Utilities|Time|SetTimerbyEvent (delegate Custom|CustomEvent) 3e+02 true))))))

(fn ConstructionScript)