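; Learning Agents interactor that defines and exchanges observations and actions for BP_AStarPawn agents.
; Observations combine pawn location, a direction derived from that location, target location and eight surrounding raycast points, all relative to the pawn's transform.
; The Forward action drives movement input, but wall contact overrides it with a stronger push away from the wall.
; A Rotation action is specified but never applied.
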(fn SpecifyAgentObservation
  (params (InObservationSchema :type Learning%20Agents%20Observation%20Schema%20Object%20Reference))
  (return (Class|LearningAgentsObservations|SpecifyStructObservation InObservationSchema (Utilities|Map|MakeMap "Pawn" (Class|LearningAgentsObservations|SpecifyStructObservation InObservationSchema (Utilities|Map|MakeMap "Location" (Class|LearningAgentsObservations|SpecifyLocationObservation InObservationSchema 1e+02) "Direction" (Class|LearningAgentsObservations|SpecifyDirectionObservation InObservationSchema))) "Target" (Class|LearningAgentsObservations|SpecifyLocationObservation InObservationSchema 1e+02) "Rays" (Class|LearningAgentsObservations|SpecifyStaticArrayObservation InObservationSchema (Class|LearningAgentsObservations|SpecifyLocationObservation InObservationSchema 1e+02) 8)))))

(fn GatherAgentObservation
  (params (InObservationObject :type Learning%20Agents%20Observation%20Object%20Object%20Reference) (AgentId :type Integer))
  (LocalVariables|SetObsActor (Class|LearningAgentsManagerListener|GetAgent AgentId "/Game/Blueprints/BP_AStarPawn.BP_AStarPawn_C"))
  (Utilities|FlowControl|Sequence
    (:then_0
      (Utilities|Array|Clear (LocalVariables|GetWallLocations))
      (for _index (range 0 7)
        (Utilities|Array|Add (LocalVariables|GetWallLocations) (Class|LearningAgentsObservations|MakeLocationObservation InObservationObject (Utilities|Array|Get(acopy) (Default|Raycast (LocalVariables|GetObsActor) (Utilities|Array|MakeArray 0.0 9e+01 -9e+01 45.0 -45.0 135.0 -135.0 1.8e+02) 5e+02) _index) (Transformation|GetActorTransform (LocalVariables|GetObsActor)) "LocationObservation" false 0))))
    (:then_1
      (return (Class|LearningAgentsObservations|MakeStructObservation InObservationObject (Utilities|Map|MakeMap "Pawn" (Class|LearningAgentsObservations|MakeStructObservation InObservationObject (Utilities|Map|MakeMap "Location" (Class|LearningAgentsObservations|MakeLocationObservation InObservationObject (Pawn|GetNavAgentLocation (LocalVariables|GetObsActor)) (Transformation|GetActorTransform (LocalVariables|GetObsActor)) "LocationObservation" true 0) "Direction" (Class|LearningAgentsObservations|MakeDirectionObservation InObservationObject (Pawn|GetNavAgentLocation (LocalVariables|GetObsActor)) (Transformation|GetActorTransform (LocalVariables|GetObsActor)) "DirectionObservation" true 0))) "Target" (Class|LearningAgentsObservations|MakeLocationObservation InObservationObject (Variables|/Game/Blueprints/BP_AStarPawn.BP_AStarPawn_C|GetTargetLocation (LocalVariables|GetObsActor)) (Transformation|GetActorTransform (LocalVariables|GetObsActor)) "LocationObservation" false 0) "Rays" (Class|LearningAgentsObservations|MakeStaticArrayObservation InObservationObject (LocalVariables|GetWallLocations))))))))

(fn SpecifyAgentAction
  (params (InActionSchema :type Learning%20Agents%20Action%20Schema%20Object%20Reference))
  (return (Class|LearningAgentsActions|SpecifyStructAction InActionSchema (Utilities|Map|MakeMap "Rotation" (Class|LearningAgentsActions|SpecifyRotationAction InActionSchema 9e+01 "Rotation") "Forward" (Class|LearningAgentsActions|SpecifyDirectionAction InActionSchema "Forward")))))

(fn PerformAgentAction
  (params (InActionObject :type Learning%20Agents%20Action%20Object%20Object%20Reference) (InActionObjectElement :type Learning%20Agents%20Action%20Object%20Element%20Structure%20%28by%20ref%29) (AgentId :type Integer))
  (LocalVariables|SetActActor (Class|LearningAgentsManagerListener|GetAgent AgentId "/Game/Blueprints/BP_AStarPawn.BP_AStarPawn_C"))
  (Variables|/Game/Blueprints/BP_AStarPawn.BP_AStarPawn_C|SetLastLocation (LocalVariables|GetActActor) (Pawn|GetNavAgentLocation (LocalVariables|GetActActor)))
  (bind _outelements (Class|LearningAgentsActions|GetStructAction InActionObject InActionObjectElement))
  (if (not (Variables|/Game/Blueprints/BP_AStarPawn.BP_AStarPawn_C|GetTouchingWall (LocalVariables|GetActActor)))
    (bind _outdirection (Class|LearningAgentsActions|GetDirectionAction InActionObject (.Value (Utilities|Map|Find _outelements "Forward")) (Transformation|GetActorTransform (LocalVariables|GetActActor)) "Forward" false 0))
    (Pawn|Input|AddMovementInput (LocalVariables|GetActActor) (Math|Vector|MakeVector (.x _outdirection) (.y _outdirection) 0.0) 1.0 false)
    (else
      (Pawn|Input|AddMovementInput (LocalVariables|GetActActor) (Math|Vector|MakeVector (.x (Math|Vector|Normalize (- (Transformation|GetActorLocation (LocalVariables|GetActActor)) (Variables|/Game/Blueprints/BP_AStarPawn.BP_AStarPawn_C|GetTouchingWallLocation (LocalVariables|GetActActor))))) (.y (Math|Vector|Normalize (- (Transformation|GetActorLocation (LocalVariables|GetActActor)) (Variables|/Game/Blueprints/BP_AStarPawn.BP_AStarPawn_C|GetTouchingWallLocation (LocalVariables|GetActActor))))) 0.0) 2.0 false))))