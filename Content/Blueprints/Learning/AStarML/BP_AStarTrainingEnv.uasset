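; Learning Agents training environment that scores and resets BP_AStarPawn agents learning to reach a target location.
; Reward combines 2D progress since the last location, a small step penalty, tiered proximity bonuses, an arrival bonus and a wall-contact penalty, and is printed on each evaluation.
; Episodes truncate on reaching the target and terminate on touching a wall.
; Reset delegates to the pawn to move to a new start location.
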(fn GatherAgentReward
  (params (AgentId :type Integer))
  (LocalVariables|SetRewardActor (Class|LearningAgentsManagerListener|GetAgent AgentId "/Game/Blueprints/AStarBPs/BP_AStarPawn.BP_AStarPawn_C"))
  (Development|PrintString 0 (Utilities|String|ToString(Float) (+ (Class|LearningAgentsRewards|MakeReward (- (Math|Vector|Distance2D(Vector) (Variables|/Game/Blueprints/AStarBPs/BP_AStarPawn.BP_AStarPawn_C|GetLastLocation (LocalVariables|GetRewardActor)) (Variables|/Game/Blueprints/AStarBPs/BP_AStarPawn.BP_AStarPawn_C|GetTargetLocation (LocalVariables|GetRewardActor))) (Math|Vector|Distance2D(Vector) (Pawn|GetNavAgentLocation (LocalVariables|GetRewardActor)) (Variables|/Game/Blueprints/AStarBPs/BP_AStarPawn.BP_AStarPawn_C|GetTargetLocation (LocalVariables|GetRewardActor)))) 0.1 "Reward" false 0) (Class|LearningAgentsRewards|MakeReward -0.001 1.0 "Reward" false 0) (Class|LearningAgentsRewards|MakeRewardonLocationDifferenceBelowThreshold (Pawn|GetNavAgentLocation (LocalVariables|GetRewardActor)) (Variables|/Game/Blueprints/AStarBPs/BP_AStarPawn.BP_AStarPawn_C|GetTargetLocation (LocalVariables|GetRewardActor)) 5e+02 1.0 "LocationDifferenceBelowThresholdReward" false 0) (Class|LearningAgentsRewards|MakeRewardonCondition (Utilities|Operators|EqualEqual (Pawn|GetNavAgentLocation (LocalVariables|GetRewardActor)) (Variables|/Game/Blueprints/AStarBPs/BP_AStarPawn.BP_AStarPawn_C|GetTargetLocation (LocalVariables|GetRewardActor)) 1e+02) 1e+01 "ConditionReward" false 0) (Class|LearningAgentsRewards|MakeRewardonCondition (== (Variables|/Game/Blueprints/AStarBPs/BP_AStarPawn.BP_AStarPawn_C|GetTouchingWall (LocalVariables|GetRewardActor)) true) -1.0 "ConditionReward" false 0) (Class|LearningAgentsRewards|MakeRewardonLocationDifferenceBelowThreshold (Pawn|GetNavAgentLocation (LocalVariables|GetRewardActor)) (Variables|/Game/Blueprints/AStarBPs/BP_AStarPawn.BP_AStarPawn_C|GetTargetLocation (LocalVariables|GetRewardActor)) 2.5e+02 5.0 "LocationDifferenceBelowThresholdReward" false 0) (Class|LearningAgentsRewards|MakeRewardonLocationDifferenceBelowThreshold (Pawn|GetNavAgentLocation (LocalVariables|GetRewardActor)) (Variables|/Game/Blueprints/AStarBPs/BP_AStarPawn.BP_AStarPawn_C|GetTargetLocation (LocalVariables|GetRewardActor)) 1.5e+02 7.5 "LocationDifferenceBelowThresholdReward" false 0))))
  (return (+ (Class|LearningAgentsRewards|MakeReward (- (Math|Vector|Distance2D(Vector) (Variables|/Game/Blueprints/AStarBPs/BP_AStarPawn.BP_AStarPawn_C|GetLastLocation (LocalVariables|GetRewardActor)) (Variables|/Game/Blueprints/AStarBPs/BP_AStarPawn.BP_AStarPawn_C|GetTargetLocation (LocalVariables|GetRewardActor))) (Math|Vector|Distance2D(Vector) (Pawn|GetNavAgentLocation (LocalVariables|GetRewardActor)) (Variables|/Game/Blueprints/AStarBPs/BP_AStarPawn.BP_AStarPawn_C|GetTargetLocation (LocalVariables|GetRewardActor)))) 0.1 "Reward" false 0) (Class|LearningAgentsRewards|MakeReward -0.001 1.0 "Reward" false 0) (Class|LearningAgentsRewards|MakeRewardonLocationDifferenceBelowThreshold (Pawn|GetNavAgentLocation (LocalVariables|GetRewardActor)) (Variables|/Game/Blueprints/AStarBPs/BP_AStarPawn.BP_AStarPawn_C|GetTargetLocation (LocalVariables|GetRewardActor)) 5e+02 1.0 "LocationDifferenceBelowThresholdReward" false 0) (Class|LearningAgentsRewards|MakeRewardonCondition (Utilities|Operators|EqualEqual (Pawn|GetNavAgentLocation (LocalVariables|GetRewardActor)) (Variables|/Game/Blueprints/AStarBPs/BP_AStarPawn.BP_AStarPawn_C|GetTargetLocation (LocalVariables|GetRewardActor)) 1e+02) 1e+01 "ConditionReward" false 0) (Class|LearningAgentsRewards|MakeRewardonCondition (== (Variables|/Game/Blueprints/AStarBPs/BP_AStarPawn.BP_AStarPawn_C|GetTouchingWall (LocalVariables|GetRewardActor)) true) -1.0 "ConditionReward" false 0) (Class|LearningAgentsRewards|MakeRewardonLocationDifferenceBelowThreshold (Pawn|GetNavAgentLocation (LocalVariables|GetRewardActor)) (Variables|/Game/Blueprints/AStarBPs/BP_AStarPawn.BP_AStarPawn_C|GetTargetLocation (LocalVariables|GetRewardActor)) 2.5e+02 5.0 "LocationDifferenceBelowThresholdReward" false 0) (Class|LearningAgentsRewards|MakeRewardonLocationDifferenceBelowThreshold (Pawn|GetNavAgentLocation (LocalVariables|GetRewardActor)) (Variables|/Game/Blueprints/AStarBPs/BP_AStarPawn.BP_AStarPawn_C|GetTargetLocation (LocalVariables|GetRewardActor)) 1.5e+02 7.5 "LocationDifferenceBelowThresholdReward" false 0))))

(fn GatherAgentCompletion
  (params (AgentId :type Integer))
  (bind _returnvalue (Class|LearningAgentsManagerListener|GetAgent AgentId "/Game/Blueprints/AStarBPs/BP_AStarPawn.BP_AStarPawn_C"))
  (return (Class|LearningAgentsCompletions|Completionor (Class|LearningAgentsCompletions|MakeCompletiononCondition (Utilities|Operators|EqualEqual (Transformation|GetActorLocation _returnvalue) (Variables|/Game/Blueprints/AStarBPs/BP_AStarPawn.BP_AStarPawn_C|GetTargetLocation _returnvalue) 1e+02) "Truncation" "ConditionCompletion" true 0) (Class|LearningAgentsCompletions|MakeCompletiononCondition (Variables|/Game/Blueprints/AStarBPs/BP_AStarPawn.BP_AStarPawn_C|GetTouchingWall _returnvalue) "Termination" "ConditionCompletion" false 0))))

(fn ResetAgentEpisode
  (params (AgentId :type Integer))
  (Default|ResettoNewStartLocation (Class|LearningAgentsManagerListener|GetAgent AgentId "/Game/Blueprints/AStarBPs/BP_AStarPawn.BP_AStarPawn_C")))