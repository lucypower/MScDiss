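; Learning Agents interactor that defines what BP_CollabAStarPawn agents observe and how they move along a spline.
; Observations are the nearest spline point's location and direction relative to the pawn; eight wall raycasts are gathered but left out.
; The action schema declares Rotation and Forward, but only Forward drives movement input, replaced by a stronger push away when touching a wall.
; Each action first records the pawn's last location and spline distance.
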(fn SpecifyAgentObservation
  (params (InObservationSchema :type Learning%20Agents%20Observation%20Schema%20Object%20Reference))
  (return (Class|LearningAgentsObservations|SpecifyStructObservation InObservationSchema (Utilities|Map|MakeMap "Pawn" (Class|LearningAgentsObservations|SpecifyStructObservation InObservationSchema (Utilities|Map|MakeMap "Location" (Class|LearningAgentsObservations|SpecifyLocationAlongSplineObservation InObservationSchema 1e+02) "Direction" (Class|LearningAgentsObservations|SpecifyDirectionAlongSplineObservation InObservationSchema)))))))

(fn GatherAgentObservation
  (params (InObservationObject :type Learning%20Agents%20Observation%20Object%20Object%20Reference) (AgentId :type Integer))
  (LocalVariables|SetObsActor (Class|LearningAgentsManagerListener|GetAgent AgentId "/Game/Blueprints/BP_CollabAStarPawn.BP_CollabAStarPawn_C"))
  (Utilities|FlowControl|Sequence
    (:then_0
      (Utilities|Array|Clear (LocalVariables|GetWallLocations))
      (for _index (range 0 7)
        (Utilities|Array|Add (LocalVariables|GetWallLocations) (Class|LearningAgentsObservations|MakeLocationObservation InObservationObject (Utilities|Array|Get(acopy) (Default|Raycast (LocalVariables|GetObsActor) (Utilities|Array|MakeArray 0.0 9e+01 -9e+01 45.0 -45.0 135.0 -135.0 1.8e+02) 5e+02) _index) (Transformation|GetActorTransform (LocalVariables|GetObsActor)) "LocationObservation" false 0))))
    (:then_1
      (return (Class|LearningAgentsObservations|MakeStructObservation InObservationObject (Utilities|Map|MakeMap "Pawn" (Class|LearningAgentsObservations|MakeStructObservation InObservationObject (Utilities|Map|MakeMap "Location" (Class|LearningAgentsObservations|MakeLocationAlongSplineObservation InObservationObject (Variables|Default|GetSpline) (Class|SplineComponent|GetDistanceAlongSplineatLocation (Variables|Default|GetSpline) (Transformation|GetActorLocation (LocalVariables|GetObsActor)) "World") (Transformation|GetActorTransform (LocalVariables|GetObsActor)) "LocationAlongSplineObservation" false 0) "Direction" (Class|LearningAgentsObservations|MakeDirectionAlongSplineObservation InObservationObject (Variables|Default|GetSpline) (Class|SplineComponent|GetDistanceAlongSplineatLocation (Variables|Default|GetSpline) (Transformation|GetActorLocation (LocalVariables|GetObsActor)) "World") (Transformation|GetActorTransform (LocalVariables|GetObsActor)) "DirectionAlongSplineObservation" false 0)))))))))

(fn SpecifyAgentAction
  (params (InActionSchema :type Learning%20Agents%20Action%20Schema%20Object%20Reference))
  (return (Class|LearningAgentsActions|SpecifyStructAction InActionSchema (Utilities|Map|MakeMap "Rotation" (Class|LearningAgentsActions|SpecifyRotationAction InActionSchema 9e+01 "Rotation") "Forward" (Class|LearningAgentsActions|SpecifyDirectionAction InActionSchema "Forward")))))

(fn PerformAgentAction
  (params (InActionObject :type Learning%20Agents%20Action%20Object%20Object%20Reference) (InActionObjectElement :type Learning%20Agents%20Action%20Object%20Element%20Structure%20%28by%20ref%29) (AgentId :type Integer))
  (LocalVariables|SetActActor (Class|LearningAgentsManagerListener|GetAgent AgentId "/Game/Blueprints/BP_CollabAStarPawn.BP_CollabAStarPawn_C"))
  (Variables|/Game/Blueprints/BP_CollabAStarPawn.BP_CollabAStarPawn_C|SetLastLocation (LocalVariables|GetActActor) (Pawn|GetNavAgentLocation (LocalVariables|GetActActor)))
  (Variables|/Game/Blueprints/BP_CollabAStarPawn.BP_CollabAStarPawn_C|SetLastLocationAlongSpline (LocalVariables|GetActActor) (Class|SplineComponent|GetDistanceAlongSplineatLocation (Variables|Default|GetSpline) (Transformation|GetActorLocation (LocalVariables|GetActActor)) "World"))
  (bind _outelements (Class|LearningAgentsActions|GetStructAction InActionObject InActionObjectElement))
  (if (not (Variables|/Game/Blueprints/BP_CollabAStarPawn.BP_CollabAStarPawn_C|GetTouchingWall (LocalVariables|GetActActor)))
    (bind _outdirection (Class|LearningAgentsActions|GetDirectionAction InActionObject (.Value (Utilities|Map|Find _outelements "Forward")) (Transformation|GetActorTransform (LocalVariables|GetActActor)) "Forward" false 0))
    (Pawn|Input|AddMovementInput (LocalVariables|GetActActor) (Math|Vector|MakeVector (.x _outdirection) (.y _outdirection) 0.0) 1.0 false)
    (else
      (Pawn|Input|AddMovementInput (LocalVariables|GetActActor) (Math|Vector|MakeVector (.x (Math|Vector|Normalize (- (Transformation|GetActorLocation (LocalVariables|GetActActor)) (Variables|/Game/Blueprints/BP_CollabAStarPawn.BP_CollabAStarPawn_C|GetTouchingWallLocation (LocalVariables|GetActActor))))) (.y (Math|Vector|Normalize (- (Transformation|GetActorLocation (LocalVariables|GetActActor)) (Variables|/Game/Blueprints/BP_CollabAStarPawn.BP_CollabAStarPawn_C|GetTouchingWallLocation (LocalVariables|GetActActor))))) 0.0) 2.0 false))))