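; Manager that trains or runs a Learning Agents PPO policy for collaborative A* pawns.
; BeginPlay makes pawns tick after it, sets up the first pawn's spline, and builds interactor, policy, critic, training environment and shared-memory trainer from the spline and map generator.
; Tick runs inference or training per RunInference, which also controls network reinitialization.
; During training, a timer periodically resets the grid, pawn starts and spline.
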(event Custom|CustomEvent
  (Class|AStarMapGeneration|ResetGrid (Variables|Default|GetGridRef))
  (Default|ResettoNewStartLocation (Variables|Default|GetAStarActors))
  (Class|AStarCollabComponent|SetupSpline (Actor|GetComponentbyClass (Utilities|Array|Get(acopy) (Variables|Default|GetAStarActors)) "/Script/MScDiss.AStarCollabComponent"))
  (Utilities|FlowControl|DoOnce false) ; enters at Reset
)

(event EventBeginPlay
  (bind _shared_memory_settings (Variables|Default|GetShared%20Memory%20Settings))
  (bind _runinference (Variables|Default|GetRunInference))
  (bind _returnvalue (not _runinference))
  (Utilities|FlowControl|Sequence
    (:then_0
      (bind _outactors (Actor|GetAllActorsOfClass "/Game/Blueprints/BP_CollabAStarPawn.BP_CollabAStarPawn_C"))
      (bind _output_get (Variables|Default|SetAStarActors _outactors))
      (Actor|Tick|AddTickPrerequisiteActor _output_get self))
    (:then_1
      (bind _returnvalue_2 (Actor|GetActorOfClass "/Game/Blueprints/BP_AStarMapGen.BP_AStarMapGen_C"))
      (Variables|Default|SetGridRef _returnvalue_2))
    (:then_2
      (Utilities|FlowControl|Delay 1.0)
      (Class|AStarCollabComponent|SetupComponent (Actor|GetComponentbyClass (Utilities|Array|Get(acopy) (Variables|Default|GetAStarActors)) "/Script/MScDiss.AStarCollabComponent"))
      (Class|AStarCollabComponent|SetupSpline (Actor|GetComponentbyClass (Utilities|Array|Get(acopy) (Variables|Default|GetAStarActors)) "/Script/MScDiss.AStarCollabComponent")))
    (:then_3
      (bind _returnvalue_3 (Actor|GetActorOfClass "/Game/Blueprints/BP_Spline.BP_Spline_C"))
      (Variables|Default|SetSpline (Variables|/Game/Blueprints/BP_Spline.BP_Spline_C|GetSpline _returnvalue_3)))
    (:then_4
      (bind _returnvalue_4 (Class|LearningAgentsInteractor|MakeInteractor (Variables|Default|GetLearningAgentsManager) "/Game/Blueprints/Learning/AStarCollab/BP_AStarCollabInteractor.BP_AStarCollabInteractor_C" "AStarInteractor"))
      (bind _output_get_2 (Variables|Default|SetInteractor _returnvalue_4))
      (Variables|/Game/Blueprints/Learning/AStarCollab/BP_AStarCollabInteractor.BP_AStarCollabInteractor_C|SetSpline _output_get_2 (Variables|Default|GetSpline)))
    (:then_5
      (bind _returnvalue_5 (Class|LearningAgentsPolicy|MakePolicy (Variables|Default|GetLearningAgentsManager) (Variables|Default|GetInteractor) "/Script/LearningAgents.LearningAgentsPolicy" "AStarPolicy" "/Game/Blueprints/Learning/AStarCollab/DA_AStarEncoder.DA_AStarEncoder" "/Game/Blueprints/Learning/AStarCollab/DA_AStarPolicy.DA_AStarPolicy" "/Game/Blueprints/Learning/AStarCollab/DA_AStarDecoder.DA_AStarDecoder" _returnvalue _returnvalue _returnvalue (Variables|Default|GetPolicy%20Settings) 1234))
      (Variables|Default|SetPolicy _returnvalue_5))
    (:then_6
      (bind _returnvalue_6 (Class|LearningAgentsCritic|MakeCritic (Variables|Default|GetLearningAgentsManager) (Variables|Default|GetInteractor) (Variables|Default|GetPolicy) "/Script/LearningAgents.LearningAgentsCritic" "AStarCritic" "/Game/Blueprints/Learning/AStarCollab/DA_AStarCritic.DA_AStarCritic" (not (Variables|Default|GetRunInference)) (Variables|Default|GetCritic%20Settings) 1234))
      (Variables|Default|SetCritic _returnvalue_6))
    (:then_7
      (bind _returnvalue_7 (Class|LearningAgentsTrainingEnvironment|MakeTrainingEnvironment (Variables|Default|GetLearningAgentsManager) "/Game/Blueprints/Learning/AStarCollab/BP_AStarCollabTrainingEnv.BP_AStarCollabTrainingEnv_C" "TrainingEnvironment"))
      (bind _output_get_3 (Variables|Default|SetTrainingEnv_ _returnvalue_7))
      (Variables|/Game/Blueprints/Learning/AStarCollab/BP_AStarCollabTrainingEnv.BP_AStarCollabTrainingEnv_C|SetSpline _output_get_3 (Variables|Default|GetSpline))
      (Variables|/Game/Blueprints/Learning/AStarCollab/BP_AStarCollabTrainingEnv.BP_AStarCollabTrainingEnv_C|SetGridRef _output_get_3 (Variables|Default|GetGridRef)))
    (:then_8
      (bind _returnvalue_8 (Class|LearningAgentsCommunicatorLibrary|SpawnSharedMemoryTrainingProcess (Variables|Default|GetTrainer%20Process%20Settings) _shared_memory_settings))
      (bind _returnvalue_9 (Class|LearningAgentsCommunicatorLibrary|MakeSharedMemoryCommunicator _returnvalue_8 _shared_memory_settings))
      (Variables|Default|SetCommunicator _returnvalue_9))
    (:then_9
      (bind _returnvalue_10 (Class|LearningAgentsPPOTrainer|MakePPOTrainer (Variables|Default|GetLearningAgentsManager) (Variables|Default|GetInteractor) (Variables|Default|GetTrainingEnv_) (Variables|Default|GetPolicy) (Variables|Default|GetCritic) (Variables|Default|GetCommunicator) "/Script/LearningAgentsTraining.LearningAgentsPPOTrainer" "PPOTrainer" (Variables|Default|GetTrainer%20Settings)))
      (Variables|Default|SetPPOTrainer _returnvalue_10))
    (:then_10
      (if (Variables|Default|GetRunInference)
        (Default|ResettoNewStartLocation (Variables|Default|GetAStarActors))))))

(event EventTick
  (params (DeltaSeconds :type Float%20%28single-precision%29))
  (if (Variables|Default|GetRunInference)
    (Class|LearningAgentsPolicy|RunInference (Variables|Default|GetPolicy) 0.0)
    (else
      (Class|LearningAgentsPPOTrainer|RunTraining (Variables|Default|GetPPOTrainer) (Variables|Default|GetTrainer%20Training%20Settings) (Variables|Default|GetTraining%20Game%20Settings) true true)
      (Utilities|FlowControl|DoOnce false
        (:Completed
          (Utilities|Time|SetTimerbyEvent (delegate Custom|CustomEvent) 3e+02 true))))))

(fn ConstructionScript)