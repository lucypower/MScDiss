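; Learning Agents training environment for BP_CollabAStarPawn agents learning to follow a spline toward a target location.
; Rewards combine spline distance change and completion fraction with tiered target-proximity bonuses, penalizing straying from the spline or standing still.
; Episodes truncate on reaching the target and also end when the pawn strays off the spline or stops moving.
; Resets zero the stored spline distance and move the pawn to a new start.
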(fn GatherAgentReward
  (params (AgentId :type Integer))
  (LocalVariables|SetRewardActor (Class|LearningAgentsManagerListener|GetAgent AgentId "/Game/Blueprints/BP_CollabAStarPawn.BP_CollabAStarPawn_C"))
  (return (+ (Class|LearningAgentsRewards|MakeReward (- (Variables|/Game/Blueprints/BP_CollabAStarPawn.BP_CollabAStarPawn_C|GetLastLocationAlongSpline (LocalVariables|GetRewardActor)) (Class|SplineComponent|GetDistanceAlongSplineatLocation (Variables|Default|GetSpline) (Transformation|GetActorLocation (LocalVariables|GetRewardActor)) "World")) 1.0 "Reward" false 0) (Class|LearningAgentsRewards|MakeRewardonCondition (Utilities|Operators|EqualEqual (Pawn|GetNavAgentLocation (LocalVariables|GetRewardActor)) (Variables|/Game/Blueprints/BP_CollabAStarPawn.BP_CollabAStarPawn_C|GetTargetLocation (LocalVariables|GetRewardActor)) 1e+02) 1e+01 "ConditionReward" false 0) (Class|LearningAgentsRewards|MakeRewardonLocationDifferenceAboveThreshold (Transformation|GetActorLocation (LocalVariables|GetRewardActor)) (Spline|FindLocationClosesttoWorldLocation (Variables|Default|GetSpline) (Transformation|GetActorLocation (LocalVariables|GetRewardActor)) "World") 125.0 -1e+01 "LocationDifferenceAboveThresholdReward" false 0) (Class|LearningAgentsRewards|MakeRewardonCondition (Utilities|Operators|EqualEqual (Transformation|GetVelocity (LocalVariables|GetRewardActor)) (Math|Vector|VectorZero) 0.01) -1e+01 "ConditionReward" false 0) (Class|LearningAgentsRewards|MakeRewardonLocationDifferenceBelowThreshold (Pawn|GetNavAgentLocation (LocalVariables|GetRewardActor)) (Variables|/Game/Blueprints/BP_CollabAStarPawn.BP_CollabAStarPawn_C|GetTargetLocation (LocalVariables|GetRewardActor)) 5e+02 1.0 "LocationDifferenceBelowThresholdReward" false 0) (Class|LearningAgentsRewards|MakeRewardonLocationDifferenceBelowThreshold (Pawn|GetNavAgentLocation (LocalVariables|GetRewardActor)) (Variables|/Game/Blueprints/BP_CollabAStarPawn.BP_CollabAStarPawn_C|GetTargetLocation (LocalVariables|GetRewardActor)) 2.5e+02 5.0 "LocationDifferenceBelowThresholdReward" false 0) (Class|LearningAgentsRewards|MakeRewardonLocationDifferenceBelowThreshold (Pawn|GetNavAgentLocation (LocalVariables|GetRewardActor)) (Variables|/Game/Blueprints/BP_CollabAStarPawn.BP_CollabAStarPawn_C|GetTargetLocation (LocalVariables|GetRewardActor)) 1.5e+02 7.5 "LocationDifferenceBelowThresholdReward" false 0) (Class|LearningAgentsRewards|MakeReward (Math|Float|Clamp(Float) (/ (Class|SplineComponent|GetDistanceAlongSplineatLocation (Variables|Default|GetSpline) (Transformation|GetActorLocation (LocalVariables|GetRewardActor)) "World") (Spline|GetSplineLength (Variables|Default|GetSpline)))) 1.0 "Reward" false 0))))

(fn GatherAgentCompletion
  (params (AgentId :type Integer))
  (bind _returnvalue (Class|LearningAgentsManagerListener|GetAgent AgentId "/Game/Blueprints/BP_CollabAStarPawn.BP_CollabAStarPawn_C"))
  (bind _returnvalue_2 (Transformation|GetActorLocation _returnvalue))
  (return (Class|LearningAgentsCompletions|Completionor (Class|LearningAgentsCompletions|MakeCompletiononCondition (Utilities|Operators|EqualEqual (Transformation|GetActorLocation _returnvalue) (Variables|/Game/Blueprints/BP_CollabAStarPawn.BP_CollabAStarPawn_C|GetTargetLocation _returnvalue) 1.5e+02) "Truncation" "ConditionCompletion" true 0) (Class|LearningAgentsCompletions|MakeCompletiononLocationDifferenceAboveThreshold (Spline|FindLocationClosesttoWorldLocation (Variables|Default|GetSpline) _returnvalue_2 "World") _returnvalue_2 125.0 "Termination" "LocationDifferenceAboveThresholdCompletion" false 0) (Class|LearningAgentsCompletions|MakeCompletiononCondition (Utilities|Operators|EqualEqual (Transformation|GetVelocity _returnvalue) (Math|Vector|VectorZero) 0.01) "Termination" "ConditionCompletion" false 0))))

(fn ResetAgentEpisode
  (params (AgentId :type Integer))
  (bind _returnvalue (Class|LearningAgentsManagerListener|GetAgent AgentId "/Game/Blueprints/BP_CollabAStarPawn.BP_CollabAStarPawn_C"))
  (Variables|/Game/Blueprints/BP_CollabAStarPawn.BP_CollabAStarPawn_C|SetLastLocationAlongSpline _returnvalue 0.0)
  (Default|ResettoNewStartLocation _returnvalue))